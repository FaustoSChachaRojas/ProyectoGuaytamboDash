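; BP_Skybox is a skybox actor that follows the player's RunCharacter and blends its material from game mode state.
; Each Tick it moves to the character's location, then reads ProbabilidadSkybox from OurGSGameMode into the material's Interpolacion scalar parameter.
; It calls CreateDynamicMaterialInstance on the static mesh every frame rather than caching an instance.
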(event EventBeginPlay)

(event Collision|EventActorBeginOverlap
  (params (OtherActor :type Actor%20Object%20Reference)))

(event EventTick
  (params (DeltaSeconds :type Float%20%28single-precision%29))
  (bind _staticmesh (Variables|Default|GetStaticMesh))
  (bind _asrun_character (Utilities|Casting|CastToRunCharacter (Game|Player|GetPlayerPawn 0)))
  (Transformation|SetActorLocation (Transformation|GetActorLocation _asrun_character) false false)
  (bind _asour_gsgame_mode (Utilities|Casting|CastToOurGSGameMode (Game|GetGameMode)))
  (bind _returnvalue (Rendering|Material|CreateDynamicMaterialInstance _staticmesh 0 (Rendering|Material|GetMaterial _staticmesh 0) "None" :!class /Script/Engine.PrimitiveComponent))
  (Rendering|Material|SetScalarParameterValue _returnvalue "Interpolacion" (Variables|/Game/AuthenticationUI/OurGSGameMode.OurGSGameMode_C|GetProbabilidadSkybox _asour_gsgame_mode) :!class /Script/Engine.MaterialInstanceDynamic))

(fn ConstructionScript)