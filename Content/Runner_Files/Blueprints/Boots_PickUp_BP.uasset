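; Jump boots pickup actor that temporarily boosts the runner character's jump height.
; On overlap with a RunCharacter it raises the character movement jump velocity and hides the Boot component.
; After a ten-second delay it resets the jump velocity on player 0's character, rather than the stored overlapping one, then destroys itself.
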(event Collision|EventActorBeginOverlap
  (params (OtherActor :type Actor%20Object%20Reference))
  (bind _asrun_character (Utilities|Casting|CastToRunCharacter OtherActor))
  (Variables|/Script/Engine.CharacterMovementComponent|SetJumpZVelocity (Variables|/Script/Engine.Character|GetCharacterMovement _asrun_character) 1.2e+03)
  (Rendering|SetVisibility (Variables|Default|Getboot) false false)
  (Utilities|FlowControl|Delay 1e+01)
  (bind _asrun_character_2 (Utilities|Casting|CastToRunCharacter (Game|GetPlayerCharacter 0)))
  (Variables|/Script/Engine.CharacterMovementComponent|SetJumpZVelocity (Variables|/Script/Engine.Character|GetCharacterMovement _asrun_character_2) 6e+02)
  (Actor|DestroyActor))

(fn ConstructionScript)