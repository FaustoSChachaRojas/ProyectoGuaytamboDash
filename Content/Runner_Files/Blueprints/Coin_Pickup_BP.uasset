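; Coin pickup for the runner that adds one to the coin count on the game mode, with a sound.
; Touching the coin collects and destroys it immediately.
; When the runner's magnet is active, the larger sphere collects it early and flags it against double counting.
; A timeline then pulls it toward the player via VInterpTo plus a Slide offset until destruction after a short delay.
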(event OnComponentBeginOverlap(BigSphere)
  (params (OverlappedComponent :type Primitive%20Component%20Object%20Reference) (OtherActor :type Actor%20Object%20Reference) (OtherComp :type Primitive%20Component%20Object%20Reference) (OtherBodyIndex :type Integer) (bFromSweep :type Boolean) (SweepResult :type Hit%20Result%20Structure%20%28by%20ref%29))
  (bind _asrun_character (Utilities|Casting|CastToRunCharacter OtherActor))
  (if (Variables|/Game/RunnerPersonBP/Blueprints/RunCharacter.RunCharacter_C|GetMagnetActive _asrun_character)
    (Utilities|FlowControl|Sequence
      (:then_0
        (bind _asour_gsgame_mode (Utilities|Casting|CastToOurGSGameMode (Game|GetGameMode)))
        (Math|Integer|IncrementInt (Variables|/Game/AuthenticationUI/OurGSGameMode.OurGSGameMode_C|GetCoins _asour_gsgame_mode)
          (:%20%20
            (Variables|Default|SetUsed_in_BigSphere true)
            (Audio|SpawnSound2D "/Game/Runner_Files/SFX/Pickup_SFX.Pickup_SFX" 1.0 1.0 0.0 0)
            (Utilities|FlowControl|Delay 1.0)
            (Actor|DestroyActor))))
      (:then_1
        (bind _slide (Timeline|Timeline_0 PlayFromStart)
          (:Update
            (Transformation|SetActorLocation (+ _slide (Math|Interpolation|VInterpTo (.Location (Math|Transform|BreakTransform (Transformation|GetActorTransform))) (Transformation|GetActorLocation (Game|GetPlayerCharacter 0)) (Utilities|Time|GetWorldDeltaSeconds) 15.0)) false false)))))))

(event OnComponentBeginOverlap(Coin)
  (params (OverlappedComponent :type Primitive%20Component%20Object%20Reference) (OtherActor :type Actor%20Object%20Reference) (OtherComp :type Primitive%20Component%20Object%20Reference) (OtherBodyIndex :type Integer) (bFromSweep :type Boolean) (SweepResult :type Hit%20Result%20Structure%20%28by%20ref%29))
  (Utilities|Casting|CastToRunCharacter OtherActor)
  (bind _asour_gsgame_mode (Utilities|Casting|CastToOurGSGameMode (Game|GetGameMode)))
  (if (not (Variables|Default|GetUsed_in_BigSphere))
    (Variables|/Game/AuthenticationUI/OurGSGameMode.OurGSGameMode_C|SetCoins _asour_gsgame_mode (+ (Variables|/Game/AuthenticationUI/OurGSGameMode.OurGSGameMode_C|GetCoins _asour_gsgame_mode) 1))
    (Audio|SpawnSound2D "/Game/Runner_Files/SFX/Pickup_SFX.Pickup_SFX" 1.0 1.0 0.0 0)
    (Actor|DestroyActor)))

(fn ConstructionScript)