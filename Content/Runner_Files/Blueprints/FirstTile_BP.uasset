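; Opening track tile for an endless runner with three lanes.
; When the runner overlaps its box, it has the game mode spawn another tile, adds points, doubles walk speed within a clamp, then destroys itself after a short delay.
; SpawnObstacles, not called in this Blueprint, randomly places pipes, rocks, coins, magnets or boots per lane.
; Each check rerolls separately, and an empty lane skips the lanes after it.
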(event OnComponentBeginOverlap(Box)
  (params (OverlappedComponent :type Primitive%20Component%20Object%20Reference) (OtherActor :type Actor%20Object%20Reference) (OtherComp :type Primitive%20Component%20Object%20Reference) (OtherBodyIndex :type Integer) (bFromSweep :type Boolean) (SweepResult :type Hit%20Result%20Structure%20%28by%20ref%29))
  (Utilities|Casting|CastToRunCharacter OtherActor)
  (bind _asour_gsgame_mode (Utilities|Casting|CastToOurGSGameMode (Game|GetGameMode)))
  (Default|SpawnTile _asour_gsgame_mode)
  (bind _asour_gsgame_mode_2 (Utilities|Casting|CastToOurGSGameMode (Game|GetGameMode)))
  (Variables|/Game/AuthenticationUI/OurGSGameMode.OurGSGameMode_C|SetCurrentPoint _asour_gsgame_mode_2 (+ 5 (Variables|/Game/AuthenticationUI/OurGSGameMode.OurGSGameMode_C|GetCurrentPoint _asour_gsgame_mode_2)))
  (bind _asrun_character (Utilities|Casting|CastToRunCharacter (Game|GetPlayerCharacter 0)))
  (Variables|/Script/Engine.CharacterMovementComponent|SetMaxWalkSpeed (Variables|/Script/Engine.Character|GetCharacterMovement _asrun_character) (Math|Float|Clamp(Float) (* (Variables|/Script/Engine.CharacterMovementComponent|GetMaxWalkSpeed (Variables|/Script/Engine.Character|GetCharacterMovement _asrun_character)) 2.0) 6e+02 1.2e+03))
  (Utilities|FlowControl|Delay 0.5)
  (Actor|DestroyActor))

(event EventBeginPlay)

(fn ConstructionScript)

(fn SpawnObstacles
  (bind _returnvalue (Math|Random|RandomFloatinRange 0.0 1.0))
  (bind _returnvalue_2 (Math|Random|RandomFloatinRange 0.0 1.0))
  (bind _returnvalue_3 (Math|Random|RandomFloatinRange 0.0 1.0))
  (bind _lane1 (Variables|Default|Getlane1))
  (bind _lane2 (Variables|Default|Getlane2))
  (bind _lane0 (Variables|Default|Getlane0))
  (bind _returnvalue_4 (Transformation|GetWorldTransform _lane2))
  (bind _returnvalue_5 (Transformation|GetWorldTransform _lane0))
  (bind _returnvalue_6 (Transformation|GetWorldTransform _lane1))
  ;[1 1 1] Lane 0
  (if (Math|Float|InRange(Float) _returnvalue_2 0.0 0.4)
    (Game|SpawnActorfromClass "/Game/Runner_Files/Blueprints/Obstacle_Pipe_BP.Obstacle_Pipe_BP_C" _returnvalue_5 "Undefined" 0 0)
    ;[1 1 1] Lane 1
    (if (Math|Float|InRange(Float) _returnvalue_3 0.0 0.4) :!label _label
      (Game|SpawnActorfromClass "/Game/Runner_Files/Blueprints/Obstacle_Pipe_BP.Obstacle_Pipe_BP_C" _returnvalue_6 "Undefined" 0 0)
      ;[1 1 1] Lane 2
      (if (Math|Float|InRange(Float) _returnvalue 0.0 0.4) :!label _label_2
        (Game|SpawnActorfromClass "/Game/Runner_Files/Blueprints/Obstacle_Pipe_BP.Obstacle_Pipe_BP_C" _returnvalue_4 "Undefined" 0 0)
        (elif (Math|Float|InRange(Float) _returnvalue 0.4 0.5)
          (Game|SpawnActorfromClass "/Game/Runner_Files/Blueprints/Obstacle_Rock_BP.Obstacle_Rock_BP_C" _returnvalue_4 "Undefined" 0 0)
          (elif (Math|Float|InRange(Float) _returnvalue 0.5 0.95)
            (Game|SpawnActorfromClass "/Game/Runner_Files/Blueprints/Coin_Pickup_BP.Coin_Pickup_BP_C" _returnvalue_4 "Undefined" 0 0)
            (elif (Math|Float|InRange(Float) _returnvalue 0.975 1.0)
              (Game|SpawnActorfromClass "/Game/Runner_Files/Blueprints/Magnet_PickUp_BP.Magnet_PickUp_BP_C" _returnvalue_4 "Undefined" 0 0)
              (elif (Math|Float|InRange(Float) _returnvalue 0.975 1.0)
                (Game|SpawnActorfromClass "/Game/Runner_Files/Blueprints/Boots_PickUp_BP.Boots_PickUp_BP_C" _returnvalue_4 "Undefined" 0 0))))))
      (elif (Math|Float|InRange(Float) _returnvalue_3 0.4 0.5)
        (Game|SpawnActorfromClass "/Game/Runner_Files/Blueprints/Obstacle_Rock_BP.Obstacle_Rock_BP_C" _returnvalue_6 "Undefined" 0 0)
        (goto _label_2)
        (elif (Math|Float|InRange(Float) _returnvalue_3 0.5 0.95)
          (Game|SpawnActorfromClass "/Game/Runner_Files/Blueprints/Coin_Pickup_BP.Coin_Pickup_BP_C" _returnvalue_6 "Undefined" 0 0)
          (goto _label_2)
          (elif (Math|Float|InRange(Float) _returnvalue_3 0.975 1.0)
            (Game|SpawnActorfromClass "/Game/Runner_Files/Blueprints/Magnet_PickUp_BP.Magnet_PickUp_BP_C" _returnvalue_6 "Undefined" 0 0)
            (goto _label_2)
            (elif (Math|Float|InRange(Float) _returnvalue_3 0.975 1.0)
              (Game|SpawnActorfromClass "/Game/Runner_Files/Blueprints/Boots_PickUp_BP.Boots_PickUp_BP_C" _returnvalue_6 "Undefined" 0 0)
              (goto _label_2))))))
    (elif (Math|Float|InRange(Float) _returnvalue_2 0.4 0.5)
      (Game|SpawnActorfromClass "/Game/Runner_Files/Blueprints/Obstacle_Rock_BP.Obstacle_Rock_BP_C" _returnvalue_5 "Undefined" 0 0)
      (goto _label)
      (elif (Math|Float|InRange(Float) _returnvalue_2 0.5 0.95)
        (Game|SpawnActorfromClass "/Game/Runner_Files/Blueprints/Coin_Pickup_BP.Coin_Pickup_BP_C" _returnvalue_5 "Undefined" 0 0)
        (goto _label)
        (elif (Math|Float|InRange(Float) _returnvalue_2 0.95 0.975)
          (Game|SpawnActorfromClass "/Game/Runner_Files/Blueprints/Magnet_PickUp_BP.Magnet_PickUp_BP_C" _returnvalue_5 "Undefined" 0 0)
          (goto _label)
          (elif (Math|Float|InRange(Float) _returnvalue_2 0.975 1.0)
            (Game|SpawnActorfromClass "/Game/Runner_Files/Blueprints/Boots_PickUp_BP.Boots_PickUp_BP_C" _returnvalue_5 "Undefined" 0 0)
            (goto _label)))))))