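; Boots pickup for the runner game that temporarily raises the RunCharacter's jump height.
; On overlap it boosts JumpZVelocity and hides the boot mesh, then after a ten-second delay restores the jump velocity on the player character and destroys itself.
; The first time, tracked by the character's BootHud flag, it also pauses the game and shows the BootHud widget.
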(event Collision|EventActorBeginOverlap
  (params (OtherActor :type Actor%20Object%20Reference))
  (bind _asrun_character (Utilities|Casting|CastToRunCharacter OtherActor))
  (Variables|/Script/Engine.CharacterMovementComponent|SetJumpZVelocity (Variables|/Script/Engine.Character|GetCharacterMovement _asrun_character) 9e+02)
  (Utilities|FlowControl|Sequence
    (:then_0
      (Rendering|SetVisibility (Variables|Default|Getboot) false false)
      (Utilities|FlowControl|Delay 1e+01)
      (bind _asrun_character_2 (Utilities|Casting|CastToRunCharacter (Game|GetPlayerCharacter 0)))
      (Variables|/Script/Engine.CharacterMovementComponent|SetJumpZVelocity (Variables|/Script/Engine.Character|GetCharacterMovement _asrun_character_2) 6e+02)
      (Actor|DestroyActor))
    (:then_1
      (if (not (Variables|/Game/RunnerPersonBP/Blueprints/RunCharacter.RunCharacter_C|GetBootHud _asrun_character))
        (Game|SetGamePaused true)
        (bind _returnvalue (UserInterface|CreateWidget "/Game/Runner_Files/UI/RaymiÑam/HUD-TUTO/BootHud.BootHud_C"))
        (UserInterface|Viewport|AddtoViewport _returnvalue 0)
        (bind _asrun_character_3 (Utilities|Casting|CastToRunCharacter (Game|GetPlayerCharacter 0)))
        (Variables|/Game/RunnerPersonBP/Blueprints/RunCharacter.RunCharacter_C|SetBootHud _asrun_character_3 true)))))

(fn ConstructionScript)