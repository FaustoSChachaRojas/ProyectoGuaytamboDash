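; Magnet power-up pickup for the runner that switches on the player's coin magnet and its timer bar.
; On overlap it sets MagnetActive on RunCharacter, resets the GameInstance timer and hides its mesh; its zero-time destroy check follows that reset, so fails.
; Tick calls the character's EventBarraIman while the bar flag is set.
; A GameInstance flag limits the game-pausing ImanHud popup to the first pickup.
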(event Collision|EventActorBeginOverlap
  (params (OtherActor :type Actor%20Object%20Reference))
  (bind _asrun_character (Utilities|Casting|CastToRunCharacter OtherActor))
  (Utilities|FlowControl|Sequence
    (:then_0
      (Variables|/Game/RunnerPersonBP/Blueprints/RunCharacter.RunCharacter_C|SetMagnetActive _asrun_character true)
      (bind _asinstance_hud (Utilities|Casting|CastToInstanceHud (Game|GetGameInstance)))
      (Variables|/Game/Runner_Files/UI/RaymiÑam/InstanceHud.InstanceHud_C|SetBarraIman _asinstance_hud true)
      (Variables|/Game/Runner_Files/UI/RaymiÑam/InstanceHud.InstanceHud_C|SetTiempoIman _asinstance_hud 1.0)
      (Rendering|SetVisibility (Variables|Default|GetCoin) false false)
      (if (== (Variables|/Game/Runner_Files/UI/RaymiÑam/InstanceHud.InstanceHud_C|GetTiempoIman _asinstance_hud) 0.0)
        (Actor|DestroyActor)))
    (:then_1
      (bind _asinstance_hud_2 (Utilities|Casting|CastToInstanceHud (Game|GetGameInstance)))
      (if (Math|Boolean|Equal(Boolean) (Variables|/Game/Runner_Files/UI/RaymiÑam/InstanceHud.InstanceHud_C|GetDesactiveHudsIman _asinstance_hud_2) false)
        (Game|SetGamePaused true)
        (bind _returnvalue (UserInterface|CreateWidget "/Game/Runner_Files/UI/RaymiÑam/HUD-AYUDA/ImanHud.ImanHud_C"))
        (UserInterface|Viewport|AddtoViewport _returnvalue 0)
        (Utilities|Casting|CastToRunCharacter (Game|GetPlayerCharacter 0))
        (Variables|/Game/Runner_Files/UI/RaymiÑam/InstanceHud.InstanceHud_C|SetDesactiveHudsIman _asinstance_hud_2 true)))))

(event EventTick
  (params (DeltaSeconds :type Float%20%28single-precision%29))
  (bind _asinstance_hud (Utilities|Casting|CastToInstanceHud (Game|GetGameInstance)))
  (if (Variables|/Game/Runner_Files/UI/RaymiÑam/InstanceHud.InstanceHud_C|GetBarraIman _asinstance_hud)
    (bind _asrun_character (Utilities|Casting|CastToRunCharacter (Game|GetPlayerCharacter 0)))
    (Default|EventBarraIman _asrun_character)))

(fn ConstructionScript)