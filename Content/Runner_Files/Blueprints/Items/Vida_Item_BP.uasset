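; Life pickup item for the runner game that raises the player's Vida count when overlapped.
; Any actor overlap increments Vida on the InstanceHud game instance, plays a sound and destroys the item.
; If DesactiveHudsVida is still false, it also pauses the game, shows the VidaHud widget and sets that flag, so the popup does not repeat on later pickups.
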(event EventBeginPlay)

(event EventTick
  (params (DeltaSeconds :type Float%20%28single-precision%29)))

(event Collision|EventActorBeginOverlap
  (params (OtherActor :type Actor%20Object%20Reference))
  (bind _asinstance_hud (Utilities|Casting|CastToInstanceHud (Game|GetGameInstance)))
  (Utilities|FlowControl|Sequence
    (:then_0
      (bind _result (Math|Integer|IncrementInt (Variables|/Game/Runner_Files/UI/RaymiÑam/InstanceHud.InstanceHud_C|GetVida _asinstance_hud))
        (:%20%20
          (Variables|/Game/Runner_Files/UI/RaymiÑam/InstanceHud.InstanceHud_C|SetVida _asinstance_hud _result)
          (Audio|PlaySound2D "/Game/Runner_Files/Sonido/Items-Obstaculos/Item.Item" 1.0 1.0 0.0 0 0)
          (Actor|DestroyActor))))
    (:then_1
      (if (Math|Boolean|Equal(Boolean) (Variables|/Game/Runner_Files/UI/RaymiÑam/InstanceHud.InstanceHud_C|GetDesactiveHudsVida _asinstance_hud) false)
        (Game|SetGamePaused true)
        (bind _returnvalue (UserInterface|CreateWidget "/Game/Runner_Files/UI/RaymiÑam/HUD-AYUDA/VidaHud.VidaHud_C"))
        (UserInterface|Viewport|AddtoViewport _returnvalue 0)
        (Variables|/Game/Runner_Files/UI/RaymiÑam/InstanceHud.InstanceHud_C|SetDesactiveHudsVida _asinstance_hud true)))))

(fn ConstructionScript)