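; Endless-runner floor tile that dresses itself randomly and keeps the track growing.
; On BeginPlay it offsets floor UVs and adds debris or vegetation, rocks and houses at side guides, using GameMode mesh and color arrays with dynamic materials.
; Its trigger box spawns a curve or the next tile, the latter also raising score and runner speed, then destroys this tile after a delay.
; SpawnObstacles is never called.
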(event OnComponentBeginOverlap(Box_SpawnTile)
  (params (OverlappedComponent :type Primitive%20Component%20Object%20Reference) (OtherActor :type Actor%20Object%20Reference) (OtherComp :type Primitive%20Component%20Object%20Reference) (OtherBodyIndex :type Integer) (bFromSweep :type Boolean) (SweepResult :type Hit%20Result%20Structure%20%28by%20ref%29))
  (bind _asrun_character (Utilities|Casting|CastToRunCharacter OtherActor))
  (bind _asour_gsgame_mode (Utilities|Casting|CastToOurGSGameMode (Game|GetGameMode)))
  (Default|GenerarCurvas _asour_gsgame_mode)
  (if (or (Variables|/Game/RunnerPersonBP/Blueprints/RunCharacter.RunCharacter_C|GetCambiarPisoCurvoIzquierda _asrun_character) (Variables|/Game/RunnerPersonBP/Blueprints/RunCharacter.RunCharacter_C|GetCambiarPisoCurvoDerecha _asrun_character))
    (if (Variables|/Game/RunnerPersonBP/Blueprints/RunCharacter.RunCharacter_C|GetCambiarPisoCurvoDerecha _asrun_character)
      (Game|SpawnActorfromClass "/Game/Runner_Files/Blueprints/PisoCurvaDerecha_BP.PisoCurvaDerecha_BP_C" (Variables|/Game/AuthenticationUI/OurGSGameMode.OurGSGameMode_C|GetNextSpawnPoint _asour_gsgame_mode) "Undefined" 0 0)
      (Utilities|FlowControl|Delay 5.0)
      (Actor|DestroyActor)
      (else
        (Game|SpawnActorfromClass "/Game/Runner_Files/Blueprints/PisoCurvaIzquierda_BP.PisoCurvaIzquierda_BP_C" (Variables|/Game/AuthenticationUI/OurGSGameMode.OurGSGameMode_C|GetNextSpawnPoint _asour_gsgame_mode) "Undefined" 0 0)
        (Utilities|FlowControl|Delay 5.0)
        (Actor|DestroyActor)))
    (else
      (Default|SpawnTile _asour_gsgame_mode)
      (bind _asour_gsgame_mode_2 (Utilities|Casting|CastToOurGSGameMode (Game|GetGameMode)))
      (Variables|/Game/AuthenticationUI/OurGSGameMode.OurGSGameMode_C|SetCurrentPoint _asour_gsgame_mode_2 (+ 5 (Variables|/Game/AuthenticationUI/OurGSGameMode.OurGSGameMode_C|GetCurrentPoint _asour_gsgame_mode_2)))
      (bind _asrun_character_2 (Utilities|Casting|CastToRunCharacter (Game|GetPlayerCharacter 0)))
      (Variables|/Script/Engine.CharacterMovementComponent|SetMaxWalkSpeed (Variables|/Script/Engine.Character|GetCharacterMovement _asrun_character_2) (Math|Float|Clamp(Float) (* (Variables|/Script/Engine.CharacterMovementComponent|GetMaxWalkSpeed (Variables|/Script/Engine.Character|GetCharacterMovement _asrun_character_2)) 1.001) 6e+02 2e+04))
      (Utilities|FlowControl|Delay 5.0)
      (Actor|DestroyActor))))

(event OnComponentEndOverlap(Floor)
  (params (OverlappedComponent :type Primitive%20Component%20Object%20Reference) (OtherActor :type Actor%20Object%20Reference) (OtherComp :type Primitive%20Component%20Object%20Reference) (OtherBodyIndex :type Integer))
  (Utilities|Casting|CastToRunCharacter OtherActor)
  (Development|PrintString "Hello"))

(event EventBeginPlay
  (CallFunction|OffsetMaterialPisoMaster) ; Se cambia el offset de la textura(aun por definir)para que se vea mejor
  (CallFunction|ControlFlujoEscombrosVegetacion)
  (CallFunction|GenerarRocas)
  (CallFunction|GenerarCasas))

(fn ConstructionScript)

(fn SpawnObstacles
  (bind _returnvalue (Math|Random|RandomFloatinRange -5e+02 5e+02))
  ;[1 1 1] Lane 0
  (Game|SpawnActorfromClass "/Game/Runner_Files/Blueprints/Obstacle_Rock_BP.Obstacle_Rock_BP_C" (Math|Transform|MakeTransform (+ (.location (Transformation|GetWorldTransform (Variables|Default|GetGuiaObstaculos))) (Math|Vector|MakeVector _returnvalue _returnvalue 0.0)) "0, 0, 0" "1,1,1") "Undefined" 0 0))

(fn GenerarEscombrosVegetacion
  (params (Malla :type Static%20Mesh%20Object%20Reference) (NumSpawn :type Integer))
  (bind _returnvalue (Math|Random|RandomFloatinRange 1.0 2.0))
  (bind _asour_gsgame_mode (Utilities|Casting|CastToOurGSGameMode (Game|GetGameMode)))
  (for _index (range 0 1) ; Se escoge cada guia
    (if (== _index 0)
      (Variables|Script|SetGuiaTemp_Escombros (Variables|Default|GetGuiaEscombros_RocasIZQ))
      (Variables|Script|SetDistanciaGuiaEscombros 5e+02)
      (for _index_2 (range 1 NumSpawn) :!label _label ; POr cada guia se spawnea 4 veces
        (bind _returnvalue_2 (AddComponent|AddStaticMeshComponent false (Math|Transform|MakeTransform (Math|Vector|MakeVector (+ (Math|Random|RandomFloatinRange 0.0 1e+03) (.x (.location (Transformation|GetRelativeTransform (Variables|Script|GetGuiaTemp_Escombros))))) (+ (Math|Random|RandomFloatinRange 0.0 (Variables|Script|GetDistanciaGuiaEscombros)) (.y (.location (Transformation|GetRelativeTransform (Variables|Script|GetGuiaTemp_Escombros))))) 0.0) (Math|Rotator|MakeRotator 0.0 0.0 (Math|Random|RandomFloatinRange 0.0 3.6e+02)) (Math|Vector|MakeVector _returnvalue _returnvalue _returnvalue))))
        (Components|StaticMesh|SetStaticMesh _returnvalue_2 Malla)
        (bind _returnvalue_3 (Rendering|Material|CreateDynamicMaterialInstance _returnvalue_2 0 (Rendering|Material|GetMaterial _returnvalue_2 0) "None" :!class /Script/Engine.PrimitiveComponent))
        (Rendering|Material|SetVectorParameterValue _returnvalue_3 "FactorColor" (Math|Conversions|ToLinearColor(Color) (Utilities|Array|Get(acopy) (Variables|/Game/AuthenticationUI/OurGSGameMode.OurGSGameMode_C|GetColores_Escombros _asour_gsgame_mode) (Math|Random|RandomIntegerinRange 0 (- (Utilities|Array|Length (Variables|/Game/AuthenticationUI/OurGSGameMode.OurGSGameMode_C|GetColores_Escombros _asour_gsgame_mode)) 1)))) :!class /Script/Engine.MaterialInstanceDynamic) ; se cambia el color de las mallas
      )
      (elif (== _index 1)
        (Variables|Script|SetGuiaTemp_Escombros (Variables|Default|GetGuiaEscombros_RocasDER))
        (Variables|Script|SetDistanciaGuiaEscombros -5e+02)
        (goto _label)))))

(fn GenerarCasas
  (bind _asour_gsgame_mode (Utilities|Casting|CastToOurGSGameMode (Game|GetGameMode)))
  (for _index (range 0 5) ; Se actualiza la locacion de la casa en cada guia
    (if (== _index 0)
      (Variables|Script|SetGuiaTemp_CasasRuinas (Variables|Default|GetGuia1CasasIZQ))
      (bind _returnvalue (AddComponent|AddStaticMeshComponent false (Math|Transform|MakeTransform (.location (Transformation|GetRelativeTransform (Variables|Script|GetGuiaTemp_CasasRuinas))) (Math|Rotator|MakeRotator 0.0 0.0 (Math|Conversions|ToFloat(Integer) (Utilities|Array|Get(acopy) (Variables|Script|GetGirosPerpendiculares_CasasRuinas) (Math|Random|RandomIntegerinRange 0 3)))) (.scale (Transformation|GetRelativeTransform (Variables|Script|GetGuiaTemp_CasasRuinas)))) :!label _label))
      (bind _returnvalue_2 (Components|StaticMesh|SetStaticMesh _returnvalue (.malla (Utilities|Array|Get(acopy) (Variables|/Game/AuthenticationUI/OurGSGameMode.OurGSGameMode_C|GetCasas_Strc _asour_gsgame_mode) (Math|Random|RandomIntegerinRange 0 (- (Utilities|Array|Length (Variables|/Game/AuthenticationUI/OurGSGameMode.OurGSGameMode_C|GetCasas_Strc _asour_gsgame_mode)) 1))))))
      (if _returnvalue_2
        (bind _returnvalue_3 (Rendering|Material|CreateDynamicMaterialInstance _returnvalue 0 (Rendering|Material|GetMaterial _returnvalue 0) "None" :!class /Script/Engine.PrimitiveComponent))
        (Rendering|Material|SetVectorParameterValue _returnvalue_3 "FactorColor" (Math|Conversions|ToLinearColor(Color) (Utilities|Array|Get(acopy) (Variables|/Game/AuthenticationUI/OurGSGameMode.OurGSGameMode_C|GetColores_CasasRuinas _asour_gsgame_mode) (Math|Random|RandomIntegerinRange 0 (- (Utilities|Array|Length (Variables|/Game/AuthenticationUI/OurGSGameMode.OurGSGameMode_C|GetColores_CasasRuinas _asour_gsgame_mode)) 1)))) :!class /Script/Engine.MaterialInstanceDynamic))
      (elif (== _index 1)
        (Variables|Script|SetGuiaTemp_CasasRuinas (Variables|Default|GetGuia2CasasIZQ))
        (goto _label)
        (elif (== _index 2)
          (Variables|Script|SetGuiaTemp_CasasRuinas (Variables|Default|GetGuia3CasasIZQ))
          (goto _label)
          (elif (== _index 3)
            (Variables|Script|SetGuiaTemp_CasasRuinas (Variables|Default|GetGuia1CasasDER))
            (goto _label)
            (elif (== _index 4)
              (Variables|Script|SetGuiaTemp_CasasRuinas (Variables|Default|GetGuia2CasasDER))
              (goto _label)
              (elif (== _index 5)
                (Variables|Script|SetGuiaTemp_CasasRuinas (Variables|Default|GetGuia3CasasDER))
                (goto _label)))))))))

(fn GenerarRocas
  (bind _returnvalue (Math|Random|RandomFloatinRange 1.0 4.0))
  (bind _asour_gsgame_mode (Utilities|Casting|CastToOurGSGameMode (Game|GetGameMode)))
  (bind _aparicion_ (CallFunction|ProbabilidadAparecimiento (.nivelprobabilidad (Utilities|Array|Get(acopy) (Variables|/Game/AuthenticationUI/OurGSGameMode.OurGSGameMode_C|GetRocas_Strc _asour_gsgame_mode) (Math|Random|RandomIntegerinRange 0 (- (Utilities|Array|Length (Variables|/Game/AuthenticationUI/OurGSGameMode.OurGSGameMode_C|GetRocas_Strc _asour_gsgame_mode)) 1))))))
  (if _aparicion_
    (for _index (range 0 1)
      (if (== _index 0)
        (Variables|Script|SetGuiaTemp_Rocas (Variables|Default|GetGuiaEscombros_RocasIZQ))
        (for _index_2 (range 1 (Math|Random|RandomIntegerinRange (.x (.numspawn (Utilities|Array|Get(acopy) (Variables|/Game/AuthenticationUI/OurGSGameMode.OurGSGameMode_C|GetRocas_Strc _asour_gsgame_mode) (Math|Random|RandomIntegerinRange 0 (- (Utilities|Array|Length (Variables|/Game/AuthenticationUI/OurGSGameMode.OurGSGameMode_C|GetRocas_Strc _asour_gsgame_mode)) 1))))) (.y (.numspawn (Utilities|Array|Get(acopy) (Variables|/Game/AuthenticationUI/OurGSGameMode.OurGSGameMode_C|GetRocas_Strc _asour_gsgame_mode) (Math|Random|RandomIntegerinRange 0 (- (Utilities|Array|Length (Variables|/Game/AuthenticationUI/OurGSGameMode.OurGSGameMode_C|GetRocas_Strc _asour_gsgame_mode)) 1))))))) :!label _label
          (bind _returnvalue_2 (AddComponent|AddStaticMeshComponent false (Math|Transform|MakeTransform (Math|Vector|MakeVector (+ (Math|Random|RandomFloatinRange 0.0 1e+03) (.x (.location (Transformation|GetRelativeTransform (Variables|Script|GetGuiaTemp_Rocas))))) (+ (Math|Random|RandomFloatinRange -3e+02 3e+02) (.y (.location (Transformation|GetRelativeTransform (Variables|Script|GetGuiaTemp_Rocas))))) 0.0) (Math|Rotator|MakeRotator 0.0 0.0 (Math|Random|RandomFloatinRange 0.0 3.6e+02)) (Math|Vector|MakeVector _returnvalue _returnvalue _returnvalue))))
          (Components|StaticMesh|SetStaticMesh _returnvalue_2 (.malla (Utilities|Array|Get(acopy) (Variables|/Game/AuthenticationUI/OurGSGameMode.OurGSGameMode_C|GetRocas_Strc _asour_gsgame_mode) (Math|Random|RandomIntegerinRange 0 (- (Utilities|Array|Length (Variables|/Game/AuthenticationUI/OurGSGameMode.OurGSGameMode_C|GetRocas_Strc _asour_gsgame_mode)) 1)))))
          (bind _returnvalue_3 (Rendering|Material|CreateDynamicMaterialInstance _returnvalue_2 0 (Rendering|Material|GetMaterial _returnvalue_2 0) "None" :!class /Script/Engine.PrimitiveComponent))
          (Rendering|Material|SetVectorParameterValue _returnvalue_3 "FactorColor" (Math|Conversions|ToLinearColor(Color) (Utilities|Array|Get(acopy) (Variables|/Game/AuthenticationUI/OurGSGameMode.OurGSGameMode_C|GetColores_Escombros _asour_gsgame_mode) (Math|Random|RandomIntegerinRange 0 (- (Utilities|Array|Length (Variables|/Game/AuthenticationUI/OurGSGameMode.OurGSGameMode_C|GetColores_Escombros _asour_gsgame_mode)) 1)))) :!class /Script/Engine.MaterialInstanceDynamic))
        (elif (== _index 1)
          (Variables|Script|SetGuiaTemp_Rocas (Variables|Default|GetGuiaEscombros_RocasDER))
          (goto _label))))))

(fn OffsetMaterialPisoMaster
  (bind _floor (Variables|Default|GetFloor))
  (bind _returnvalue (Rendering|Material|CreateDynamicMaterialInstance _floor 0 (Rendering|Material|GetMaterial _floor 0) "None" :!class /Script/Engine.PrimitiveComponent))
  (Rendering|Material|SetVectorParameterValue _returnvalue "DesplazamientoUV" (Utilities|Struct|MakeLinearColor (Math|Random|RandomFloatinRange 0.0 1.0) 0.0 0.0 1.0) :!class /Script/Engine.MaterialInstanceDynamic))

(fn ProbabilidadAparecimiento
  (params (NivelProbabildiad :type Float%20%28single-precision%29))
  (return (Math|Float|InRange(Float) (Math|Random|RandomFloatinRange 0.0 1.0) 0.0 NivelProbabildiad)))

(fn ControlFlujoEscombrosVegetacion
  (bind _asour_gsgame_mode (Utilities|Casting|CastToOurGSGameMode (Game|GetGameMode)))
  (Development|PrintString (Utilities|String|ToString(Float) (.nivelprobabilidad (Utilities|Array|Get(acopy) (Variables|/Game/AuthenticationUI/OurGSGameMode.OurGSGameMode_C|GetEscombros_Strc _asour_gsgame_mode) (Math|Random|RandomIntegerinRange 0 (- (Utilities|Array|Length (Variables|/Game/AuthenticationUI/OurGSGameMode.OurGSGameMode_C|GetEscombros_Strc _asour_gsgame_mode)) 1))))) true true "(R=0.361714,G=1.000000,B=0.000000,A=1.000000)")
  (if (Math|Float|InRange(Float) (Math|Random|RandomFloatinRange 0.0 1.0) 0.0 (.nivelprobabilidad (Utilities|Array|Get(acopy) (Variables|/Game/AuthenticationUI/OurGSGameMode.OurGSGameMode_C|GetEscombros_Strc _asour_gsgame_mode) (Math|Random|RandomIntegerinRange 0 (- (Utilities|Array|Length (Variables|/Game/AuthenticationUI/OurGSGameMode.OurGSGameMode_C|GetEscombros_Strc _asour_gsgame_mode)) 1)))))
    (CallFunction|GenerarEscombrosVegetacion (.malla (Utilities|Array|Get(acopy) (Variables|/Game/AuthenticationUI/OurGSGameMode.OurGSGameMode_C|GetEscombros_Strc _asour_gsgame_mode) (Math|Random|RandomIntegerinRange 0 (- (Utilities|Array|Length (Variables|/Game/AuthenticationUI/OurGSGameMode.OurGSGameMode_C|GetEscombros_Strc _asour_gsgame_mode)) 1)))) (Math|Random|RandomIntegerinRange (.x (.numspawn (Utilities|Array|Get(acopy) (Variables|/Game/AuthenticationUI/OurGSGameMode.OurGSGameMode_C|GetEscombros_Strc _asour_gsgame_mode) (Math|Random|RandomIntegerinRange 0 (- (Utilities|Array|Length (Variables|/Game/AuthenticationUI/OurGSGameMode.OurGSGameMode_C|GetEscombros_Strc _asour_gsgame_mode)) 1))))) (.y (.numspawn (Utilities|Array|Get(acopy) (Variables|/Game/AuthenticationUI/OurGSGameMode.OurGSGameMode_C|GetEscombros_Strc _asour_gsgame_mode) (Math|Random|RandomIntegerinRange 0 (- (Utilities|Array|Length (Variables|/Game/AuthenticationUI/OurGSGameMode.OurGSGameMode_C|GetEscombros_Strc _asour_gsgame_mode)) 1)))))))
    (else
      (CallFunction|GenerarEscombrosVegetacion (.malla (Utilities|Array|Get(acopy) (Variables|/Game/AuthenticationUI/OurGSGameMode.OurGSGameMode_C|GetVegetacion_Strc _asour_gsgame_mode) (Math|Random|RandomIntegerinRange 0 (- (Utilities|Array|Length (Variables|/Game/AuthenticationUI/OurGSGameMode.OurGSGameMode_C|GetVegetacion_Strc _asour_gsgame_mode)) 1)))) (Math|Random|RandomIntegerinRange (.x (.numspawn (Utilities|Array|Get(acopy) (Variables|/Game/AuthenticationUI/OurGSGameMode.OurGSGameMode_C|GetVegetacion_Strc _asour_gsgame_mode) (Math|Random|RandomIntegerinRange 0 (- (Utilities|Array|Length (Variables|/Game/AuthenticationUI/OurGSGameMode.OurGSGameMode_C|GetVegetacion_Strc _asour_gsgame_mode)) 1))))) (.y (.numspawn (Utilities|Array|Get(acopy) (Variables|/Game/AuthenticationUI/OurGSGameMode.OurGSGameMode_C|GetVegetacion_Strc _asour_gsgame_mode) (Math|Random|RandomIntegerinRange 0 (- (Utilities|Array|Length (Variables|/Game/AuthenticationUI/OurGSGameMode.OurGSGameMode_C|GetVegetacion_Strc _asour_gsgame_mode)) 1))))))))))