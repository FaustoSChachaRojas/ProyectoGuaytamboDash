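; Rock obstacle for a runner game that kills the player character on contact.
; On BeginPlay it randomizes its pitch and yaw and scales the Roca component independently on each axis for visual variety.
; It destroys itself after a fixed delay.
; Overlapping a RunCharacter calls that character's DeathFunction.
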(event EventBeginPlay
  (bind _returnvalue (Math|Random|RandomFloatinRange 1.0 5.0))
  (Transformation|SetActorRotation (Math|Rotator|MakeRotator 0.0 (Math|Random|RandomFloatinRange 0.0 1e+01) (Math|Random|RandomFloatinRange 0.0 3.6e+02)))
  (Transformation|SetRelativeScale3D (Variables|Default|GetRoca) (Math|Vector|MakeVector _returnvalue _returnvalue _returnvalue))
  (Utilities|FlowControl|Delay 15.0)
  (Actor|DestroyActor))

(event Collision|EventActorBeginOverlap
  (params (OtherActor :type Actor%20Object%20Reference))
  (bind _asrun_character (Utilities|Casting|CastToRunCharacter OtherActor))
  (Default|DeathFunction _asrun_character))

(event EventTick
  (params (DeltaSeconds :type Float%20%28single-precision%29)))

(fn ConstructionScript)