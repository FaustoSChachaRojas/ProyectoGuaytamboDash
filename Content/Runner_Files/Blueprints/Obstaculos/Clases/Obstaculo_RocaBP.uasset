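; Falling rock obstacle for the runner game that kills the player on contact while it is still moving.
; On BeginPlay it tints the rock with a random color through a dynamic material and applies a downward force.
; A delayed check from Tick turns off physics simulation once the rock's velocity reaches zero.
; Hits on three boxes by a RunCharacter call the player's DeathFunction only if the rock has nonzero velocity.
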(event OnComponentHit(Box2)
  (params (HitComponent :type Primitive%20Component%20Object%20Reference) (OtherActor :type Actor%20Object%20Reference) (OtherComp :type Primitive%20Component%20Object%20Reference) (NormalImpulse :type Vector :default "0, 0, 0") (Hit :type Hit%20Result%20Structure%20%28by%20ref%29))
  (Utilities|Casting|CastToRunCharacter OtherActor)
  (if (not (Math|Vector|Equal(Vector) (Transformation|GetComponentVelocity (Variables|Default|GetRoca)) "0, 0, 0" 0.0001))
    (bind _asrun_character (Utilities|Casting|CastToRunCharacter (Game|Player|GetPlayerPawn 0)))
    (Default|DeathFunction _asrun_character)))

(event OnComponentHit(Box1)
  (params (HitComponent :type Primitive%20Component%20Object%20Reference) (OtherActor :type Actor%20Object%20Reference) (OtherComp :type Primitive%20Component%20Object%20Reference) (NormalImpulse :type Vector :default "0, 0, 0") (Hit :type Hit%20Result%20Structure%20%28by%20ref%29))
  (Utilities|Casting|CastToRunCharacter OtherActor)
  (if (not (Math|Vector|Equal(Vector) (Transformation|GetComponentVelocity (Variables|Default|GetRoca)) "0, 0, 0" 0.0001))
    (bind _asrun_character (Utilities|Casting|CastToRunCharacter (Game|Player|GetPlayerPawn 0)))
    (Default|DeathFunction _asrun_character)))

(event OnComponentHit(Box)
  (params (HitComponent :type Primitive%20Component%20Object%20Reference) (OtherActor :type Actor%20Object%20Reference) (OtherComp :type Primitive%20Component%20Object%20Reference) (NormalImpulse :type Vector :default "0, 0, 0") (Hit :type Hit%20Result%20Structure%20%28by%20ref%29))
  (Utilities|Casting|CastToRunCharacter OtherActor)
  (if (not (Math|Vector|Equal(Vector) (Transformation|GetComponentVelocity (Variables|Default|GetRoca)) "0, 0, 0" 0.0001))
    (bind _asrun_character (Utilities|Casting|CastToRunCharacter (Game|Player|GetPlayerPawn 0)))
    (Default|DeathFunction _asrun_character)))

(event EventBeginPlay
  (bind _colores (Variables|Default|GetColores))
  (bind _roca (Variables|Default|GetRoca))
  (bind _returnvalue (Rendering|Material|CreateDynamicMaterialInstance _roca 0 (Rendering|Material|GetMaterial _roca 0) "None" :!class /Script/Engine.PrimitiveComponent))
  (Rendering|Material|SetVectorParameterValue _returnvalue "FactorColor" (Math|Conversions|ToLinearColor(Color) (Utilities|Array|Get(acopy) _colores (Math|Random|RandomIntegerinRange 0 (- (Utilities|Array|Length _colores) 1)))) :!class /Script/Engine.MaterialInstanceDynamic)
  (Physics|AddForce (Variables|Default|GetRoca) "0.000000, 0,-1500.000000" "None" false)
  (Utilities|FlowControl|Delay 8.0))

(event EventTick
  (params (DeltaSeconds :type Float%20%28single-precision%29))
  (Utilities|FlowControl|Delay 0.05)
  (if (Math|Vector|Equal(Vector) (Transformation|GetComponentVelocity (Variables|Default|GetRoca)) "0, 0, 0" 0.0001)
    (Physics|SetSimulatePhysics (Variables|Default|GetRoca) false)))

(fn ConstructionScript)