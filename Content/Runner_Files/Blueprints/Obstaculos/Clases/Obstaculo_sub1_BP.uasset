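; Runner obstacle Blueprint that kills the player character on contact.
; The construction script passes the Mallas array to CambiarMalla, which sets the Pipe component to a randomly picked static mesh.
; Actor overlap casts the other actor to RunCharacter and calls its DeathFunction.
; A timed self-destroy chain is present but unconnected, so it never runs.
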(event EventBeginPlay)

(event Collision|EventActorBeginOverlap
  (params (OtherActor :type Actor%20Object%20Reference))
  (bind _asrun_character (Utilities|Casting|CastToRunCharacter OtherActor))
  (Default|DeathFunction _asrun_character))

(fn ConstructionScript
  (CallFunction|CambiarMalla (Variables|Default|GetMallas)))

(fn CambiarMalla
  (params (Arreglo :type Array%20of%20Static%20Mesh%20Object%20References))
  (Components|StaticMesh|SetStaticMesh (Variables|Default|GetPipe) (.OutItem (Utilities|Array|Random Arreglo))))