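; Child Blueprint of a character obstacle in the runner game, built around a marching cachiporrero (baton major) that kills the player on contact.
; Each tick it moves its collision Box to the root_x socket of the CachiporreroJMarchando11GUIACOLLISION component, so the hitbox follows that component.
; When the Box overlaps a RunCharacter it calls that character's DeathFunction, while actor-level overlaps pass to the parent.
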(event OnComponentBeginOverlap(Box)
  (params (OverlappedComponent :type Primitive%20Component%20Object%20Reference) (OtherActor :type Actor%20Object%20Reference) (OtherComp :type Primitive%20Component%20Object%20Reference) (OtherBodyIndex :type Integer) (bFromSweep :type Boolean) (SweepResult :type Hit%20Result%20Structure%20%28by%20ref%29))
  (bind _asrun_character (Utilities|Casting|CastToRunCharacter OtherActor))
  (Default|DeathFunction _asrun_character))

(event EventBeginPlay
  (|CallParentFunction) ; This node is disabled and will not be called.\nDrag off pins to build functionality.
)

(event Collision|EventActorBeginOverlap
  (params (OtherActor :type Actor%20Object%20Reference))
  (|CallParentFunction OtherActor))

(event EventTick
  (params (DeltaSeconds :type Float%20%28single-precision%29))
  (Transformation|SetWorldLocation (Variables|Default|GetBox) (Transformation|GetSocketLocation (Variables|Default|GetCachiporreroJ_Marchando11_GUIACOLLISION) "root_x") false false))

(fn ConstructionScript)