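; Right-turn floor tile for a procedurally generated runner map.
; On BeginPlay it sets the game mode's next spawn point and turn direction, then adds random debris and house meshes at guide components.
; Sublevel flags and probabilities in the game mode select the meshes, tinted through dynamic materials.
; When the runner overlaps the trigger, a timeline turns the control yaw, then updates the character's rotation, spawns the next tile and destroys this one after a delay.
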(event OnComponentBeginOverlap(BoxCollision_Animacion)
  (params (OverlappedComponent :type Primitive%20Component%20Object%20Reference) (OtherActor :type Actor%20Object%20Reference) (OtherComp :type Primitive%20Component%20Object%20Reference) (OtherBodyIndex :type Integer) (bFromSweep :type Boolean) (SweepResult :type Hit%20Result%20Structure%20%28by%20ref%29))
  (bind _asrun_character (Utilities|Casting|CastToRunCharacter OtherActor))
  (bind _valorcreciente (Timeline|Timeline_0 PlayFromStart)
    (:Update
      (Pawn|SetControlRotation (Game|GetPlayerController 0) (Math|Rotator|MakeRotator 0.0 0.0 (+ (* _valorcreciente 9e+01) (Variables|/Game/RunnerPersonBP/Blueprints/RunCharacter.RunCharacter_C|GetRotacionActual _asrun_character)))))
    (:Finished
      (if (== (+ (* _valorcreciente 9e+01) (Variables|/Game/RunnerPersonBP/Blueprints/RunCharacter.RunCharacter_C|GetRotacionActual _asrun_character)) 3.6e+02)
        (Variables|/Game/RunnerPersonBP/Blueprints/RunCharacter.RunCharacter_C|SetRotacionActual _asrun_character 0.0)
        (else
          (Variables|/Game/RunnerPersonBP/Blueprints/RunCharacter.RunCharacter_C|SetRotacionActual _asrun_character (+ (* _valorcreciente 9e+01) (Variables|/Game/RunnerPersonBP/Blueprints/RunCharacter.RunCharacter_C|GetRotacionActual _asrun_character)))))
      (bind _asour_gsgame_mode (Utilities|Casting|CastToOurGSGameMode (Game|GetGameMode)))
      (Default|SpawnTile _asour_gsgame_mode)
      (Utilities|FlowControl|Delay 5.0)
      (Actor|DestroyActor))))

(event EventBeginPlay
  (CallFunction|FijarPosicionSpawn) ; Para el mapa procedural
  (CallFunction|ControlFlujoSub1Sub2))

(event Collision|EventActorBeginOverlap
  (params (OtherActor :type Actor%20Object%20Reference)))

(event EventTick
  (params (DeltaSeconds :type Float%20%28single-precision%29)))

(fn ConstructionScript)

(fn FijarPosicionSpawn
  (bind _puntoaparecercd (Variables|Default|GetPuntoAparecerCD))
  (bind _asour_gsgame_mode (Utilities|Casting|CastToOurGSGameMode (Game|GetGameMode)))
  (bind _output_get (Variables|/Game/AuthenticationUI/OurGSGameMode.OurGSGameMode_C|SetDireccionGiro _asour_gsgame_mode (Math|Rotator|MakeRotator 0.0 0.0 (Math|Conversions|ToFloat(Integer) (Math|Float|Round (.Yaw (Math|Rotator|BreakRotator (Transformation|GetWorldRotation _puntoaparecercd))))))))
  (Variables|/Game/AuthenticationUI/OurGSGameMode.OurGSGameMode_C|SetNextSpawnPoint _asour_gsgame_mode (Math|Transform|MakeTransform (Transformation|GetWorldLocation _puntoaparecercd) _output_get "1,1,1"))
  (bind _asrun_character (Utilities|Casting|CastToRunCharacter (Game|GetPlayerCharacter 0)))
  (Variables|/Game/RunnerPersonBP/Blueprints/RunCharacter.RunCharacter_C|SetCambiarPisoCurvoDerecha _asrun_character false))

(fn GenerarCasas
  (params (Espacios :type EspaciosCasa%20Enum :default "NewEnumerator4") (Malla :type Static%20Mesh%20Object%20Reference) (Colores :type Array%20of%20Color%20Structures) (AplicarShader :type Boolean))
  (bind _returnvalue (Utilities|Array|Length Colores))
  (bind _returnvalue_2 (- _returnvalue 1))
  (bind _returnvalue_3 (Math|Random|RandomIntegerinRange 0 _returnvalue_2))
  (bind _output (Utilities|Array|Get(acopy) Colores _returnvalue_3))
  (bind _returnvalue_4 (Math|Conversions|ToLinearColor(Color) _output))
  (if (Utilities|Enum|Equal(Enum) Espacios "NewEnumerator4")
    (for _index (range 0 3)
      (if (== _index 0)
        (Variables|Script|SetGuiaTemp_CasasRuinas (Variables|Default|GetGuia1Casa))
        (bind _returnvalue_5 (AddComponent|AddStaticMeshComponent false (Math|Transform|MakeTransform (.location (Transformation|GetRelativeTransform (Variables|Script|GetGuiaTemp_CasasRuinas))) (Math|Rotator|MakeRotator 0.0 0.0 (Math|Conversions|ToFloat(Integer) (Utilities|Array|Get(acopy) (Variables|Script|GetGirosPerpendiculares_CasasRuinas) (Math|Random|RandomIntegerinRange 0 3)))) (.scale (Transformation|GetRelativeTransform (Variables|Script|GetGuiaTemp_CasasRuinas)))) :!label _label))
        (Rendering|SetRenderCustomDepth _returnvalue_5 AplicarShader)
        (bind _returnvalue_6 (Components|StaticMesh|SetStaticMesh _returnvalue_5 Malla))
        (if _returnvalue_6
          (bind _returnvalue_7 (Rendering|Material|CreateDynamicMaterialInstance _returnvalue_5 0 (Rendering|Material|GetMaterial _returnvalue_5 0) "None" :!class /Script/Engine.PrimitiveComponent))
          (Rendering|Material|SetVectorParameterValue _returnvalue_7 "FactorColor" _returnvalue_4 :!class /Script/Engine.MaterialInstanceDynamic))
        (elif (== _index 1)
          (Variables|Script|SetGuiaTemp_CasasRuinas (Variables|Default|GetGuia2Casa))
          (goto _label)
          (elif (== _index 2)
            (Variables|Script|SetGuiaTemp_CasasRuinas (Variables|Default|GetGuia3Casa))
            (goto _label)
            (elif (== _index 3)
              (Variables|Script|SetGuiaTemp_CasasRuinas (Variables|Default|GetGuia4Casa))
              (goto _label))))))
    (elif (Utilities|Enum|Equal(Enum) Espacios "NewEnumerator0")
      (for _index_2 (range 0 3)
        (if (== _index_2 0)
          (Variables|Script|SetGuiaTemp_CasasRuinas (Variables|Default|GetGuia1CasaSub2))
          (bind _returnvalue_8 (AddComponent|AddStaticMeshComponent false (Math|Transform|MakeTransform (.location (Transformation|GetRelativeTransform (Variables|Script|GetGuiaTemp_CasasRuinas))) (.rotation (Transformation|GetRelativeTransform (Variables|Script|GetGuiaTemp_CasasRuinas))) (.scale (Transformation|GetRelativeTransform (Variables|Script|GetGuiaTemp_CasasRuinas)))) :!label _label_2))
          (Rendering|SetRenderCustomDepth _returnvalue_8 AplicarShader)
          (bind _returnvalue_9 (Components|StaticMesh|SetStaticMesh _returnvalue_8 Malla))
          (if _returnvalue_9
            (bind _returnvalue_10 (Rendering|Material|CreateDynamicMaterialInstance _returnvalue_8 0 (Rendering|Material|GetMaterial _returnvalue_8 0) "None" :!class /Script/Engine.PrimitiveComponent))
            (Rendering|Material|SetVectorParameterValue _returnvalue_10 "FactorColor" _returnvalue_4 :!class /Script/Engine.MaterialInstanceDynamic))
          (elif (== _index_2 1)
            (Variables|Script|SetGuiaTemp_CasasRuinas (Variables|Default|GetGuia2CasaSub2))
            (goto _label_2)
            (elif (== _index_2 2)
              (Variables|Script|SetGuiaTemp_CasasRuinas (Variables|Default|GetGuia3CasaSub2))
              (goto _label_2)
              (elif (== _index_2 3)
                (Variables|Script|SetGuiaTemp_CasasRuinas (Variables|Default|GetGuia4CasaSub2))
                (goto _label_2)))))))))

(fn GenerarObjetos
  (params (Malla :type Static%20Mesh%20Object%20Reference) (NumSpawn :type Integer) (Escala :type Float%20%28single-precision%29) (AmbosLados :type Boolean) (Distancia_Spawn_Izq :type Float%20%28single-precision%29) (Distancia_Spawn_Der :type Float%20%28single-precision%29) (Colores :type Array%20of%20Color%20Structures) (AplicarShader :type Boolean))
  (for _index (range 0 2) ; Se escoge cada guia
    (if (== _index 0)
      (Variables|Script|SetGuiaTemp_Escombros (Variables|Default|GetGuiaEscombros1))
      (Variables|Script|SetIndiceDistanciasGuias 0)
      (for _index_2 (range 1 NumSpawn) :!label _label ; POr cada guia se spawnea 4 veces
        (bind _returnvalue (AddComponent|AddStaticMeshComponent false (Math|Transform|MakeTransform (Math|Vector|MakeVector (+ (Math|Random|RandomFloatinRange (.x (Utilities|Array|Get(acopy) (Variables|Script|GetDistanciasGuias) (Variables|Script|GetIndiceDistanciasGuias))) (.y (Utilities|Array|Get(acopy) (Variables|Script|GetDistanciasGuias) (Variables|Script|GetIndiceDistanciasGuias)))) (.x (.location (Transformation|GetRelativeTransform (Variables|Script|GetGuiaTemp_Escombros))))) (+ (Math|Random|RandomFloatinRange (.z (Utilities|Array|Get(acopy) (Variables|Script|GetDistanciasGuias) (Variables|Script|GetIndiceDistanciasGuias))) (.w (Utilities|Array|Get(acopy) (Variables|Script|GetDistanciasGuias) (Variables|Script|GetIndiceDistanciasGuias)))) (.y (.location (Transformation|GetRelativeTransform (Variables|Script|GetGuiaTemp_Escombros))))) 0.0) (Math|Rotator|MakeRotator 0.0 0.0 (Math|Random|RandomFloatinRange 0.0 3.6e+02)) (Math|Vector|MakeVector Escala Escala Escala))))
        (Rendering|SetRenderCustomDepth _returnvalue AplicarShader)
        (Components|StaticMesh|SetStaticMesh _returnvalue Malla)
        (bind _returnvalue_2 (Rendering|Material|CreateDynamicMaterialInstance _returnvalue 0 (Rendering|Material|GetMaterial _returnvalue 0) "None" :!class /Script/Engine.PrimitiveComponent))
        (Rendering|Material|SetVectorParameterValue _returnvalue_2 "FactorColor" (Math|Conversions|ToLinearColor(Color) (Utilities|Array|Get(acopy) Colores (Math|Random|RandomIntegerinRange 0 (- (Utilities|Array|Length Colores) 1)))) :!class /Script/Engine.MaterialInstanceDynamic) ; se cambia el color de las mallas
      )
      (elif (== _index 1)
        (Variables|Script|SetGuiaTemp_Escombros (Variables|Default|GetGuiaEscombros2))
        (Variables|Script|SetIndiceDistanciasGuias 1)
        (goto _label)
        (elif (== _index 2)
          (Variables|Script|SetGuiaTemp_Escombros (Variables|Default|GetGuiaEscombros3))
          (Variables|Script|SetIndiceDistanciasGuias 2)
          (goto _label))))))

(fn ProbabilidadAparecimiento
  (params (NivelProbabildiad :type Float%20%28single-precision%29))
  (return (Math|Float|InRange(Float) (Math|Random|RandomFloatinRange 0.0 1.0) 0.0 NivelProbabildiad)))

(fn ControlFlujoSub1Sub2
  (bind _asour_gsgame_mode (Utilities|Casting|CastToOurGSGameMode (Game|GetGameMode)))
  (Utilities|FlowControl|Sequence
    (:then_0
      (if (not (Variables|/Game/AuthenticationUI/OurGSGameMode.OurGSGameMode_C|GetObjetosSubnivel1Terminado _asour_gsgame_mode))
        ;[1 1 1] ObjetosSub1
        (for _array_element (Variables|/Game/AuthenticationUI/OurGSGameMode.OurGSGameMode_C|GetObjetosSubnivel1_Strc _asour_gsgame_mode)
          (bind _aparicion_ (CallFunction|ProbabilidadAparecimiento (Math|Float|Clamp(Float) (.NivelProbabilidad (Utilities|Struct|BreakEstructuraObjeto _array_element)) 0.0 (.ProbabilidadMaxima (Utilities|Struct|BreakEstructuraObjeto _array_element)))))
          (if _aparicion_
            (CallFunction|GenerarObjetos (.Malla (Utilities|Struct|BreakEstructuraObjeto _array_element)) (Math|Random|RandomIntegerinRange (.x (.NumSpawn (Utilities|Struct|BreakEstructuraObjeto _array_element))) (.y (.NumSpawn (Utilities|Struct|BreakEstructuraObjeto _array_element)))) (Math|Random|RandomFloatinRange (.x (.RangoEscala (Utilities|Struct|BreakEstructuraObjeto _array_element))) (.y (.RangoEscala (Utilities|Struct|BreakEstructuraObjeto _array_element)))) (.AmbosLados (Utilities|Struct|BreakEstructuraObjeto _array_element)) (.x (.Distancia_Spawn (Utilities|Struct|BreakEstructuraObjeto _array_element))) (.y (.Distancia_Spawn (Utilities|Struct|BreakEstructuraObjeto _array_element))) (.Colores (Utilities|Struct|BreakEstructuraObjeto _array_element)) (.AplicarShader (Utilities|Struct|BreakEstructuraObjeto _array_element)))))))
    (:then_1
      ;[1 1 1] ObjetosSub2
      (if (not (Variables|/Game/AuthenticationUI/OurGSGameMode.OurGSGameMode_C|GetObjetosSubnivel2Terminados _asour_gsgame_mode))
        (for _array_element_2 (Variables|/Game/AuthenticationUI/OurGSGameMode.OurGSGameMode_C|GetObjetosSubnivel2_Strc _asour_gsgame_mode)
          (bind _aparicion__2 (CallFunction|ProbabilidadAparecimiento (Math|Float|Clamp(Float) (.NivelProbabilidad (Utilities|Struct|BreakEstructuraObjeto _array_element_2)) 0.0 (.ProbabilidadMaxima (Utilities|Struct|BreakEstructuraObjeto _array_element_2)))))
          (if _aparicion__2
            (CallFunction|GenerarObjetos (.Malla (Utilities|Struct|BreakEstructuraObjeto _array_element_2)) (Math|Random|RandomIntegerinRange (.x (.NumSpawn (Utilities|Struct|BreakEstructuraObjeto _array_element_2))) (.y (.NumSpawn (Utilities|Struct|BreakEstructuraObjeto _array_element_2)))) (Math|Random|RandomFloatinRange (.x (.RangoEscala (Utilities|Struct|BreakEstructuraObjeto _array_element_2))) (.y (.RangoEscala (Utilities|Struct|BreakEstructuraObjeto _array_element_2)))) (.AmbosLados (Utilities|Struct|BreakEstructuraObjeto _array_element_2)) (.x (.Distancia_Spawn (Utilities|Struct|BreakEstructuraObjeto _array_element_2))) (.y (.Distancia_Spawn (Utilities|Struct|BreakEstructuraObjeto _array_element_2))) (.Colores (Utilities|Struct|BreakEstructuraObjeto _array_element_2)) (.AplicarShader (Utilities|Struct|BreakEstructuraObjeto _array_element_2)))))))
    (:then_2
      ;[1 1 1] Objetos Subnivel3
      (if (Variables|/Game/AuthenticationUI/OurGSGameMode.OurGSGameMode_C|GetObjetosSubnivel2Terminados _asour_gsgame_mode)
        (for _array_element_3 (Variables|/Game/AuthenticationUI/OurGSGameMode.OurGSGameMode_C|GetObjetosSubnivel3_Strc _asour_gsgame_mode)
          (bind _aparicion__3 (CallFunction|ProbabilidadAparecimiento (Math|Float|Clamp(Float) (.NivelProbabilidad (Utilities|Struct|BreakEstructuraObjeto _array_element_3)) 0.0 (.ProbabilidadMaxima (Utilities|Struct|BreakEstructuraObjeto _array_element_3)))))
          (if _aparicion__3
            (CallFunction|GenerarObjetos (.Malla (Utilities|Struct|BreakEstructuraObjeto _array_element_3)) (Math|Random|RandomIntegerinRange (.x (.NumSpawn (Utilities|Struct|BreakEstructuraObjeto _array_element_3))) (.y (.NumSpawn (Utilities|Struct|BreakEstructuraObjeto _array_element_3)))) (Math|Random|RandomFloatinRange (.x (.RangoEscala (Utilities|Struct|BreakEstructuraObjeto _array_element_3))) (.y (.RangoEscala (Utilities|Struct|BreakEstructuraObjeto _array_element_3)))) (.AmbosLados (Utilities|Struct|BreakEstructuraObjeto _array_element_3)) (.x (.Distancia_Spawn (Utilities|Struct|BreakEstructuraObjeto _array_element_3))) (.y (.Distancia_Spawn (Utilities|Struct|BreakEstructuraObjeto _array_element_3))) (.Colores (Utilities|Struct|BreakEstructuraObjeto _array_element_3)) (.AplicarShader (Utilities|Struct|BreakEstructuraObjeto _array_element_3)))))))
    (:then_3
      ;[1 1 1] Casas Sub1 a Sub2 a Sub3
      (if (Variables|/Game/AuthenticationUI/OurGSGameMode.OurGSGameMode_C|GetCasasSubnivel2Cargadas _asour_gsgame_mode)
        (bind _aparicion__4 (CallFunction|ProbabilidadAparecimiento (Variables|/Game/AuthenticationUI/OurGSGameMode.OurGSGameMode_C|GetProbabilidadCasasSubnivel2 _asour_gsgame_mode))) ; Reducir casas sub 2
        (if _aparicion__4
          (CallFunction|GenerarCasas (.espaciousado (Utilities|Array|Get(acopy) (Variables|/Game/AuthenticationUI/OurGSGameMode.OurGSGameMode_C|GetCasasSubnivel2_Strc _asour_gsgame_mode) (Math|Random|RandomIntegerinRange 0 (- (Utilities|Array|Length (Variables|/Game/AuthenticationUI/OurGSGameMode.OurGSGameMode_C|GetCasasSubnivel2_Strc _asour_gsgame_mode)) 1)))) (.malla (Utilities|Array|Get(acopy) (Variables|/Game/AuthenticationUI/OurGSGameMode.OurGSGameMode_C|GetCasasSubnivel2_Strc _asour_gsgame_mode) (Math|Random|RandomIntegerinRange 0 (- (Utilities|Array|Length (Variables|/Game/AuthenticationUI/OurGSGameMode.OurGSGameMode_C|GetCasasSubnivel2_Strc _asour_gsgame_mode)) 1)))) (.colores (Utilities|Array|Get(acopy) (Variables|/Game/AuthenticationUI/OurGSGameMode.OurGSGameMode_C|GetCasasSubnivel2_Strc _asour_gsgame_mode) (Math|Random|RandomIntegerinRange 0 (- (Utilities|Array|Length (Variables|/Game/AuthenticationUI/OurGSGameMode.OurGSGameMode_C|GetCasasSubnivel2_Strc _asour_gsgame_mode)) 1)))) (.aplicarshader (Utilities|Array|Get(acopy) (Variables|/Game/AuthenticationUI/OurGSGameMode.OurGSGameMode_C|GetCasasSubnivel2_Strc _asour_gsgame_mode) (Math|Random|RandomIntegerinRange 0 (- (Utilities|Array|Length (Variables|/Game/AuthenticationUI/OurGSGameMode.OurGSGameMode_C|GetCasasSubnivel2_Strc _asour_gsgame_mode)) 1)))) :!label _label)
          (else
            (CallFunction|GenerarCasas (.espaciousado (Utilities|Array|Get(acopy) (Variables|/Game/AuthenticationUI/OurGSGameMode.OurGSGameMode_C|GetCasasSubnivel3_Strc _asour_gsgame_mode) (Math|Random|RandomIntegerinRange 0 (- (Utilities|Array|Length (Variables|/Game/AuthenticationUI/OurGSGameMode.OurGSGameMode_C|GetCasasSubnivel3_Strc _asour_gsgame_mode)) 1)))) (.malla (Utilities|Array|Get(acopy) (Variables|/Game/AuthenticationUI/OurGSGameMode.OurGSGameMode_C|GetCasasSubnivel3_Strc _asour_gsgame_mode) (Math|Random|RandomIntegerinRange 0 (- (Utilities|Array|Length (Variables|/Game/AuthenticationUI/OurGSGameMode.OurGSGameMode_C|GetCasasSubnivel3_Strc _asour_gsgame_mode)) 1)))) (.colores (Utilities|Array|Get(acopy) (Variables|/Game/AuthenticationUI/OurGSGameMode.OurGSGameMode_C|GetCasasSubnivel3_Strc _asour_gsgame_mode) (Math|Random|RandomIntegerinRange 0 (- (Utilities|Array|Length (Variables|/Game/AuthenticationUI/OurGSGameMode.OurGSGameMode_C|GetCasasSubnivel3_Strc _asour_gsgame_mode)) 1)))) (.aplicarshader (Utilities|Array|Get(acopy) (Variables|/Game/AuthenticationUI/OurGSGameMode.OurGSGameMode_C|GetCasasSubnivel3_Strc _asour_gsgame_mode) (Math|Random|RandomIntegerinRange 0 (- (Utilities|Array|Length (Variables|/Game/AuthenticationUI/OurGSGameMode.OurGSGameMode_C|GetCasasSubnivel3_Strc _asour_gsgame_mode)) 1)))))))
        (else
          (bind _aparicion__5 (CallFunction|ProbabilidadAparecimiento (Variables|/Game/AuthenticationUI/OurGSGameMode.OurGSGameMode_C|GetProbabildiadCasasSubnivel1 _asour_gsgame_mode)))
          (if _aparicion__5
            (CallFunction|GenerarCasas "NewEnumerator4" (.malla (Utilities|Array|Get(acopy) (Variables|/Game/AuthenticationUI/OurGSGameMode.OurGSGameMode_C|GetCasasSubnivel1_Strc _asour_gsgame_mode) (Math|Random|RandomIntegerinRange 0 (- (Utilities|Array|Length (Variables|/Game/AuthenticationUI/OurGSGameMode.OurGSGameMode_C|GetCasasSubnivel1_Strc _asour_gsgame_mode)) 1)))) (.colores (Utilities|Array|Get(acopy) (Variables|/Game/AuthenticationUI/OurGSGameMode.OurGSGameMode_C|GetCasasSubnivel1_Strc _asour_gsgame_mode) (Math|Random|RandomIntegerinRange 0 (- (Utilities|Array|Length (Variables|/Game/AuthenticationUI/OurGSGameMode.OurGSGameMode_C|GetCasasSubnivel1_Strc _asour_gsgame_mode)) 1)))) (.aplicarshader (Utilities|Array|Get(acopy) (Variables|/Game/AuthenticationUI/OurGSGameMode.OurGSGameMode_C|GetCasasSubnivel1_Strc _asour_gsgame_mode) (Math|Random|RandomIntegerinRange 0 (- (Utilities|Array|Length (Variables|/Game/AuthenticationUI/OurGSGameMode.OurGSGameMode_C|GetCasasSubnivel1_Strc _asour_gsgame_mode)) 1)))))
            (else
              (goto _label))))))))