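; Left-curve floor tile for an endless runner that turns the player and extends the track.
; On BeginPlay it publishes the next spawn point and direction to OurGSGameMode, then builds random scenery from GameMode struct arrays.
; Probability-gated props scatter around three guides and houses fill four guides, tinted through dynamic material instances.
; Trigger overlap drives a Timeline rotating control yaw by -90 degrees, then requests the next tile and destroys this one after a delay.
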(event OnComponentBeginOverlap(BoxCollision_Animacion)
  (params (OverlappedComponent :type Primitive%20Component%20Object%20Reference) (OtherActor :type Actor%20Object%20Reference) (OtherComp :type Primitive%20Component%20Object%20Reference) (OtherBodyIndex :type Integer) (bFromSweep :type Boolean) (SweepResult :type Hit%20Result%20Structure%20%28by%20ref%29))
  (bind _asrun_character (Utilities|Casting|CastToRunCharacter OtherActor))
  (bind _valorcreciente (Timeline|Timeline_0 Play)
    (:Update
      (Pawn|SetControlRotation (Game|GetPlayerController 0) (Math|Rotator|MakeRotator 0.0 0.0 (+ (* _valorcreciente -9e+01) (Variables|/Game/RunnerPersonBP/Blueprints/RunCharacter.RunCharacter_C|GetRotacionActual _asrun_character)))))
    (:Finished
      (if (== (+ (* _valorcreciente -9e+01) (Variables|/Game/RunnerPersonBP/Blueprints/RunCharacter.RunCharacter_C|GetRotacionActual _asrun_character)) -3.6e+02)
        (Variables|/Game/RunnerPersonBP/Blueprints/RunCharacter.RunCharacter_C|SetRotacionActual _asrun_character 0.0)
        (else
          (Variables|/Game/RunnerPersonBP/Blueprints/RunCharacter.RunCharacter_C|SetRotacionActual _asrun_character (+ (* _valorcreciente -9e+01) (Variables|/Game/RunnerPersonBP/Blueprints/RunCharacter.RunCharacter_C|GetRotacionActual _asrun_character)))))
      (bind _asour_gsgame_mode (Utilities|Casting|CastToOurGSGameMode (Game|GetGameMode)))
      (Default|SpawnTile _asour_gsgame_mode)
      (Utilities|FlowControl|Delay 5.0)
      (Actor|DestroyActor))))

(event EventBeginPlay
  (CallFunction|FijarPosicionSpawn)
  (CallFunction|ControlFlujoSub1Sub2)
  (CallFunction|GenerarCasas))

(fn ConstructionScript)

(fn FijarPosicionSpawn
  (bind _puntoaparecerci (Variables|Default|GetPuntoAparecerCI))
  (bind _asour_gsgame_mode (Utilities|Casting|CastToOurGSGameMode (Game|GetGameMode)))
  (bind _output_get (Variables|/Game/AuthenticationUI/OurGSGameMode.OurGSGameMode_C|SetDireccionGiro _asour_gsgame_mode (Math|Rotator|MakeRotator 0.0 0.0 (Math|Conversions|ToFloat(Integer) (Math|Float|Round (.Yaw (Math|Rotator|BreakRotator (Transformation|GetWorldRotation _puntoaparecerci))))))))
  (Variables|/Game/AuthenticationUI/OurGSGameMode.OurGSGameMode_C|SetNextSpawnPoint _asour_gsgame_mode (Math|Transform|MakeTransform (Transformation|GetWorldLocation _puntoaparecerci) _output_get "1,1,1"))
  (bind _asrun_character (Utilities|Casting|CastToRunCharacter (Game|GetPlayerCharacter 0)))
  (Variables|/Game/RunnerPersonBP/Blueprints/RunCharacter.RunCharacter_C|SetCambiarPisoCurvoIzquierda _asrun_character false))

(fn GenerarObjetosSubnivel1
  (params (Malla :type Static%20Mesh%20Object%20Reference) (NumSpawn :type Integer) (Escala :type Float%20%28single-precision%29) (AmbosLados :type Boolean) (Distancia_Spawn_Izq :type Float%20%28single-precision%29) (Distancia_Spawn_Der :type Float%20%28single-precision%29) (Colores :type Array%20of%20Color%20Structures) (AplicarShader :type Boolean))
  (for _index (range 0 2) ; Se escoge cada guia
    (if (== _index 0)
      (Variables|Script|SetGuiaTemp_Escombros (Variables|Default|GetGuiaEscombros1))
      (Variables|Script|SetIndiceDistanciasGuias 0)
      (for _index_2 (range 1 NumSpawn) :!label _label ; POr cada guia se spawnea 4 veces
        (bind _returnvalue (AddComponent|AddStaticMeshComponent false (Math|Transform|MakeTransform (Math|Vector|MakeVector (+ (Math|Random|RandomFloatinRange (.x (Utilities|Array|Get(acopy) (Variables|Script|GetDistanciasGuias) (Variables|Script|GetIndiceDistanciasGuias))) (.y (Utilities|Array|Get(acopy) (Variables|Script|GetDistanciasGuias) (Variables|Script|GetIndiceDistanciasGuias)))) (.x (.location (Transformation|GetRelativeTransform (Variables|Script|GetGuiaTemp_Escombros))))) (+ (Math|Random|RandomFloatinRange (.z (Utilities|Array|Get(acopy) (Variables|Script|GetDistanciasGuias) (Variables|Script|GetIndiceDistanciasGuias))) (.w (Utilities|Array|Get(acopy) (Variables|Script|GetDistanciasGuias) (Variables|Script|GetIndiceDistanciasGuias)))) (.y (.location (Transformation|GetRelativeTransform (Variables|Script|GetGuiaTemp_Escombros))))) 0.0) (Math|Rotator|MakeRotator 0.0 0.0 (Math|Random|RandomFloatinRange 0.0 3.6e+02)) (Math|Vector|MakeVector Escala Escala Escala))))
        (Rendering|SetRenderCustomDepth _returnvalue AplicarShader)
        (Components|StaticMesh|SetStaticMesh _returnvalue Malla)
        (bind _returnvalue_2 (Rendering|Material|CreateDynamicMaterialInstance _returnvalue 0 (Rendering|Material|GetMaterial _returnvalue 0) "None" :!class /Script/Engine.PrimitiveComponent))
        (Rendering|Material|SetVectorParameterValue _returnvalue_2 "FactorColor" (Math|Conversions|ToLinearColor(Color) (Utilities|Array|Get(acopy) Colores (Math|Random|RandomIntegerinRange 0 (- (Utilities|Array|Length Colores) 1)))) :!class /Script/Engine.MaterialInstanceDynamic) ; se cambia el color de las mallas
      )
      (elif (== _index 1)
        (Variables|Script|SetGuiaTemp_Escombros (Variables|Default|GetGuiaEscombros2))
        (Variables|Script|SetIndiceDistanciasGuias 1)
        (goto _label)
        (elif (== _index 2)
          (Variables|Script|SetGuiaTemp_Escombros (Variables|Default|GetGuiaEscombros3))
          (Variables|Script|SetIndiceDistanciasGuias 2)
          (goto _label))))))

(fn ProbabilidadAparecimiento
  (params (NivelProbabildiad :type Float%20%28single-precision%29))
  (return (Math|Float|InRange(Float) (Math|Random|RandomFloatinRange 0.0 1.0) 0.0 NivelProbabildiad)))

(fn ControlFlujoSub1Sub2
  (bind _asour_gsgame_mode (Utilities|Casting|CastToOurGSGameMode (Game|GetGameMode)))
  (Utilities|FlowControl|Sequence
    (:then_0
      (for _array_element (Variables|/Game/AuthenticationUI/OurGSGameMode.OurGSGameMode_C|GetObjetosSubnivel1_Strc _asour_gsgame_mode)
        (bind _aparicion_ (CallFunction|ProbabilidadAparecimiento (.NivelProbabilidad (Utilities|Struct|BreakEstructuraBase _array_element))))
        (if _aparicion_
          (CallFunction|GenerarObjetosSubnivel1 (.Malla (Utilities|Struct|BreakEstructuraBase _array_element)) (Math|Random|RandomIntegerinRange (.x (.NumSpawn (Utilities|Struct|BreakEstructuraBase _array_element))) (.y (.NumSpawn (Utilities|Struct|BreakEstructuraBase _array_element)))) (Math|Random|RandomFloatinRange (.x (.RangoEscala (Utilities|Struct|BreakEstructuraBase _array_element))) (.y (.RangoEscala (Utilities|Struct|BreakEstructuraBase _array_element)))) (.AmbosLados (Utilities|Struct|BreakEstructuraBase _array_element)) (.x (.Distancia_Spawn (Utilities|Struct|BreakEstructuraBase _array_element))) (.y (.Distancia_Spawn (Utilities|Struct|BreakEstructuraBase _array_element))) (.Colores (Utilities|Struct|BreakEstructuraBase _array_element)) (.AplicarShader (Utilities|Struct|BreakEstructuraBase _array_element))))))
    (:then_1
      (for _array_element_2 (Variables|/Game/AuthenticationUI/OurGSGameMode.OurGSGameMode_C|GetObjetosSubnivel2_Strc _asour_gsgame_mode)
        (bind _aparicion__2 (CallFunction|ProbabilidadAparecimiento (.NivelProbabilidad (Utilities|Struct|BreakEstructuraBase _array_element_2))))
        (if _aparicion__2
          (CallFunction|GenerarObjetosSubnivel1 (.Malla (Utilities|Struct|BreakEstructuraBase _array_element_2)) (Math|Random|RandomIntegerinRange (.x (.NumSpawn (Utilities|Struct|BreakEstructuraBase _array_element_2))) (.y (.NumSpawn (Utilities|Struct|BreakEstructuraBase _array_element_2)))) (Math|Random|RandomFloatinRange (.x (.RangoEscala (Utilities|Struct|BreakEstructuraBase _array_element_2))) (.y (.RangoEscala (Utilities|Struct|BreakEstructuraBase _array_element_2)))) (.AmbosLados (Utilities|Struct|BreakEstructuraBase _array_element_2)) (.x (.Distancia_Spawn (Utilities|Struct|BreakEstructuraBase _array_element_2))) (.y (.Distancia_Spawn (Utilities|Struct|BreakEstructuraBase _array_element_2))) (.Colores (Utilities|Struct|BreakEstructuraBase _array_element_2)) (.AplicarShader (Utilities|Struct|BreakEstructuraBase _array_element_2))))))))

(fn GenerarCasas
  (bind _asour_gsgame_mode (Utilities|Casting|CastToOurGSGameMode (Game|GetGameMode)))
  (for _index (range 0 3)
    (if (== _index 0)
      (Variables|Script|SetGuiaTemp_CasasRuinas (Variables|Default|GetGuia1Casa))
      (bind _returnvalue (AddComponent|AddStaticMeshComponent false (Math|Transform|MakeTransform (.location (Transformation|GetRelativeTransform (Variables|Script|GetGuiaTemp_CasasRuinas))) (Math|Rotator|MakeRotator 0.0 0.0 (Math|Conversions|ToFloat(Integer) (Utilities|Array|Get(acopy) (Variables|Script|GetGirosPerpendiculares_CasasRuinas) (Math|Random|RandomIntegerinRange 0 3)))) (.scale (Transformation|GetRelativeTransform (Variables|Script|GetGuiaTemp_CasasRuinas)))) :!label _label))
      (Rendering|SetRenderCustomDepth _returnvalue (.aplicarshader (Utilities|Array|Get(acopy) (Variables|/Game/AuthenticationUI/OurGSGameMode.OurGSGameMode_C|GetCasasSubnivel1_Strc _asour_gsgame_mode) (Math|Random|RandomIntegerinRange 0 (- (Utilities|Array|Length (Variables|/Game/AuthenticationUI/OurGSGameMode.OurGSGameMode_C|GetCasasSubnivel1_Strc _asour_gsgame_mode)) 1)))))
      (bind _returnvalue_2 (Components|StaticMesh|SetStaticMesh _returnvalue (.malla (Utilities|Array|Get(acopy) (Variables|/Game/AuthenticationUI/OurGSGameMode.OurGSGameMode_C|GetCasasSubnivel1_Strc _asour_gsgame_mode) (Math|Random|RandomIntegerinRange 0 (- (Utilities|Array|Length (Variables|/Game/AuthenticationUI/OurGSGameMode.OurGSGameMode_C|GetCasasSubnivel1_Strc _asour_gsgame_mode)) 1))))))
      (if _returnvalue_2
        (bind _returnvalue_3 (Rendering|Material|CreateDynamicMaterialInstance _returnvalue 0 (Rendering|Material|GetMaterial _returnvalue 0) "None" :!class /Script/Engine.PrimitiveComponent))
        (Rendering|Material|SetVectorParameterValue _returnvalue_3 "FactorColor" (Math|Conversions|ToLinearColor(Color) (Utilities|Array|Get(acopy) (.colores (Utilities|Array|Get(acopy) (Variables|/Game/AuthenticationUI/OurGSGameMode.OurGSGameMode_C|GetCasasSubnivel1_Strc _asour_gsgame_mode) (Math|Random|RandomIntegerinRange 0 (- (Utilities|Array|Length (Variables|/Game/AuthenticationUI/OurGSGameMode.OurGSGameMode_C|GetCasasSubnivel1_Strc _asour_gsgame_mode)) 1)))) (Math|Random|RandomIntegerinRange 0 (- (Utilities|Array|Length (.colores (Utilities|Array|Get(acopy) (Variables|/Game/AuthenticationUI/OurGSGameMode.OurGSGameMode_C|GetCasasSubnivel1_Strc _asour_gsgame_mode) (Math|Random|RandomIntegerinRange 0 (- (Utilities|Array|Length (Variables|/Game/AuthenticationUI/OurGSGameMode.OurGSGameMode_C|GetCasasSubnivel1_Strc _asour_gsgame_mode)) 1))))) 1)))) :!class /Script/Engine.MaterialInstanceDynamic))
      (elif (== _index 1)
        (Variables|Script|SetGuiaTemp_CasasRuinas (Variables|Default|GetGuia2Casa))
        (goto _label)
        (elif (== _index 2)
          (Variables|Script|SetGuiaTemp_CasasRuinas (Variables|Default|GetGuia3Casa))
          (goto _label)
          (elif (== _index 3)
            (Variables|Script|SetGuiaTemp_CasasRuinas (Variables|Default|GetGuia4Casa))
            (goto _label)))))))