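; Right-curve floor tile for the runner, which turns the RunCharacter, requests the next tile and destroys itself after the player leaves.
; On BeginPlay it publishes the next spawn point to OurGSGameMode and randomizes its floor material.
; It then populates guide components with props and buildings, plus decals and obstacles, using GameMode sublevel flags and probabilities.
; Sublevels 1–2 use tinted mesh components for buildings, while sublevel 3 spawns attached actors.
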(event OnComponentBeginOverlap(BoxCollision_Animacion)
  (params (OverlappedComponent :type Primitive%20Component%20Object%20Reference) (OtherActor :type Actor%20Object%20Reference) (OtherComp :type Primitive%20Component%20Object%20Reference) (OtherBodyIndex :type Integer) (bFromSweep :type Boolean) (SweepResult :type Hit%20Result%20Structure%20%28by%20ref%29))
  (bind _asrun_character (Utilities|Casting|CastToRunCharacter OtherActor))
  (Default|AnimacionGiroDerecho _asrun_character)
  (bind _asour_gsgame_mode (Utilities|Casting|CastToOurGSGameMode (Game|GetGameMode)))
  (Default|SpawnTile _asour_gsgame_mode))

(event OnComponentBeginOverlap(Estadia)
  (params (OverlappedComponent :type Primitive%20Component%20Object%20Reference) (OtherActor :type Actor%20Object%20Reference) (OtherComp :type Primitive%20Component%20Object%20Reference) (OtherBodyIndex :type Integer) (bFromSweep :type Boolean) (SweepResult :type Hit%20Result%20Structure%20%28by%20ref%29))
  (Utilities|Casting|CastToRunCharacter OtherActor)
  (Variables|Script|SetEntroPersonaje true))

(event EventBeginPlay
  (Utilities|FlowControl|Sequence
    (:then_0
      (CallFunction|OffsetMaterialPisoMaster)
      (CallFunction|FijarPosicionSpawn))
    (:then_1
      (ControlCasasObjetos()|ControlCasasObjetos))
    (:then_2
      (CallFunction|SpawnDecals))
    (:then_3
      (CallFunction|ControlItems-Obstaculos))))

(event EventTick
  (params (DeltaSeconds :type Float%20%28single-precision%29))
  (bind _asrun_character (Utilities|Casting|CastToRunCharacter (Game|Player|GetPlayerPawn 0)))
  (if (not (Collision|IsOverlappingActor (Variables|Default|GetEstadia) _asrun_character :!class /Script/Engine.PrimitiveComponent))
    (if (Variables|Script|GetEntroPersonaje)
      (Utilities|FlowControl|Delay 2.0)
      (Actor|DestroyActor))))

(fn ConstructionScript)

(fn FijarPosicionSpawn
  (bind _puntoaparecercd (Variables|Default|GetPuntoAparecerCD))
  (bind _asour_gsgame_mode (Utilities|Casting|CastToOurGSGameMode (Game|GetGameMode)))
  (bind _output_get (Variables|/Game/AuthenticationUI/OurGSGameMode.OurGSGameMode_C|SetDireccionGiro _asour_gsgame_mode (Math|Rotator|MakeRotator 0.0 0.0 (Math|Conversions|ToFloat(Integer) (Math|Float|Round (.Yaw (Math|Rotator|BreakRotator (Transformation|GetWorldRotation _puntoaparecercd))))))))
  (Variables|/Game/AuthenticationUI/OurGSGameMode.OurGSGameMode_C|SetNextSpawnPoint _asour_gsgame_mode (Math|Transform|MakeTransform (Transformation|GetWorldLocation _puntoaparecercd) _output_get "1,1,1"))
  (bind _asrun_character (Utilities|Casting|CastToRunCharacter (Game|GetPlayerCharacter 0)))
  (Variables|/Game/RunnerPersonBP/Blueprints/RunCharacter.RunCharacter_C|SetCambiarPisoCurvoDerecha _asrun_character false))

(fn GenerarObjetos
  (params (Malla :type Static%20Mesh%20Object%20Reference) (NumSpawn :type Integer) (Escala :type Float%20%28single-precision%29) (AmbosLados :type Boolean) (Colores :type Array%20of%20Color%20Structures) (AplicarShader :type Boolean))
  (for _index (range 0 2) ; Se escoge cada guia
    (if (== _index 0)
      (LocalVariables|SetGuia_Temp (Variables|Default|GetGuiaObjetos1))
      (Variables|Script|SetIndiceDistanciasGuias 0)
      (for _index_2 (range 1 NumSpawn) :!label _label ; POr cada guia se spawnea 4 veces
        (bind _returnvalue (AddComponent|AddStaticMeshComponent false (Math|Transform|MakeTransform (Math|Vector|MakeVector (+ (Math|Random|RandomFloatinRange (.x (Utilities|Array|Get(acopy) (Variables|Script|GetDistanciasGuias) (Variables|Script|GetIndiceDistanciasGuias))) (.y (Utilities|Array|Get(acopy) (Variables|Script|GetDistanciasGuias) (Variables|Script|GetIndiceDistanciasGuias)))) (.x (.location (Transformation|GetRelativeTransform (LocalVariables|GetGuia_Temp))))) (+ (Math|Random|RandomFloatinRange (.z (Utilities|Array|Get(acopy) (Variables|Script|GetDistanciasGuias) (Variables|Script|GetIndiceDistanciasGuias))) (.w (Utilities|Array|Get(acopy) (Variables|Script|GetDistanciasGuias) (Variables|Script|GetIndiceDistanciasGuias)))) (.y (.location (Transformation|GetRelativeTransform (LocalVariables|GetGuia_Temp))))) 0.0) (Math|Rotator|MakeRotator 0.0 0.0 (Math|Random|RandomFloatinRange 0.0 3.6e+02)) (Math|Vector|MakeVector Escala Escala Escala))))
        (Rendering|SetRenderCustomDepth _returnvalue AplicarShader)
        (Components|StaticMesh|SetStaticMesh _returnvalue Malla)
        (bind _returnvalue_2 (Rendering|Material|CreateDynamicMaterialInstance _returnvalue 0 (Rendering|Material|GetMaterial _returnvalue 0) "None" :!class /Script/Engine.PrimitiveComponent))
        (Rendering|Material|SetVectorParameterValue _returnvalue_2 "FactorColor" (Math|Conversions|ToLinearColor(Color) (Utilities|Array|Get(acopy) Colores (Math|Random|RandomIntegerinRange 0 (- (Utilities|Array|Length Colores) 1)))) :!class /Script/Engine.MaterialInstanceDynamic) ; se cambia el color de las mallas
      )
      (elif (== _index 1)
        (LocalVariables|SetGuia_Temp (Variables|Default|GetGuiaObjetos2))
        (Variables|Script|SetIndiceDistanciasGuias 1)
        (goto _label)
        (elif (== _index 2)
          (LocalVariables|SetGuia_Temp (Variables|Default|GetGuiaObjetos3))
          (Variables|Script|SetIndiceDistanciasGuias 2)
          (goto _label))))))

(fn ProbabilidadAparecimiento
  (params (NivelProbabildiad :type Float%20%28single-precision%29))
  (return (Math|Float|InRange(Float) (Math|Random|RandomFloatinRange 0.0 1.0) 0.0 NivelProbabildiad)))

(fn OffsetMaterialPisoMaster
  (bind _pisocurvo (Variables|Default|GetPisoCurvo))
  (bind _returnvalue (Rendering|Material|CreateDynamicMaterialInstance _pisocurvo 0 (Rendering|Material|GetMaterial _pisocurvo 0) "None" :!class /Script/Engine.PrimitiveComponent))
  (Rendering|Material|SetVectorParameterValue _returnvalue "DesplazamientoUV" (Utilities|Struct|MakeLinearColor (Math|Random|RandomFloatinRange 0.0 1.0) 0.0 0.0 1.0) :!class /Script/Engine.MaterialInstanceDynamic)
  (bind _asour_gsgame_mode (Utilities|Casting|CastToOurGSGameMode (Game|GetGameMode)))
  (Rendering|Material|SetScalarParameterValue _returnvalue "Interpolacion" (Variables|/Game/AuthenticationUI/OurGSGameMode.OurGSGameMode_C|GetScalarParameterMaterial_Tiles _asour_gsgame_mode) :!class /Script/Engine.MaterialInstanceDynamic))

(fn ControlCasasObjetos
  (bind _asour_gsgame_mode (Utilities|Casting|CastToOurGSGameMode (Game|GetGameMode)))
  (Utilities|FlowControl|Sequence
    (:then_0
      ;[1 1 1] ObjetosSub1Bajada-ObjetosSub2Subida
      (if (Variables|/Game/AuthenticationUI/OurGSGameMode.OurGSGameMode_C|GetObjetosSub1_Bajada-ObjetosSub2_Subida _asour_gsgame_mode)
        (for _array_element (Variables|/Game/AuthenticationUI/OurGSGameMode.OurGSGameMode_C|GetObjetosSubnivel1_Strc _asour_gsgame_mode)
          (bind _aparicion_ (CallFunction|ProbabilidadAparecimiento (Math|Float|Clamp(Float) (.NivelProbabilidad (Utilities|Struct|BreakEstructuraObjeto _array_element)) 0.0 (.ProbabilidadMaxima (Utilities|Struct|BreakEstructuraObjeto _array_element)))))
          (if _aparicion_
            (ControlCasasObjetos()|GenerarObjetos (.Malla (Utilities|Struct|BreakEstructuraObjeto _array_element)) (Math|Random|RandomIntegerinRange (.x (.NumSpawn (Utilities|Struct|BreakEstructuraObjeto _array_element))) (.y (.NumSpawn (Utilities|Struct|BreakEstructuraObjeto _array_element)))) (Math|Random|RandomFloatinRange (.x (.RangoEscala (Utilities|Struct|BreakEstructuraObjeto _array_element))) (.y (.RangoEscala (Utilities|Struct|BreakEstructuraObjeto _array_element)))) (.AmbosLados (Utilities|Struct|BreakEstructuraObjeto _array_element)) (.Colores (Utilities|Struct|BreakEstructuraObjeto _array_element)) (.AplicarShader (Utilities|Struct|BreakEstructuraObjeto _array_element)))
            (else
              (bind _aparicion__2 (CallFunction|ProbabilidadAparecimiento (Math|Float|Clamp(Float) (.NivelProbabilidad (Utilities|Struct|BreakEstructuraObjeto (.OutItem (Utilities|Array|Random (Variables|/Game/AuthenticationUI/OurGSGameMode.OurGSGameMode_C|GetObjetosSubnivel2_Strc _asour_gsgame_mode))))) 0.0 (.ProbabilidadMaxima (Utilities|Struct|BreakEstructuraObjeto (.OutItem (Utilities|Array|Random (Variables|/Game/AuthenticationUI/OurGSGameMode.OurGSGameMode_C|GetObjetosSubnivel2_Strc _asour_gsgame_mode))))))))
              (if _aparicion__2
                (ControlCasasObjetos()|GenerarObjetos (.Malla (Utilities|Struct|BreakEstructuraObjeto (.OutItem (Utilities|Array|Random (Variables|/Game/AuthenticationUI/OurGSGameMode.OurGSGameMode_C|GetObjetosSubnivel2_Strc _asour_gsgame_mode))))) (Math|Random|RandomIntegerinRange (.x (.NumSpawn (Utilities|Struct|BreakEstructuraObjeto (.OutItem (Utilities|Array|Random (Variables|/Game/AuthenticationUI/OurGSGameMode.OurGSGameMode_C|GetObjetosSubnivel2_Strc _asour_gsgame_mode)))))) (.y (.NumSpawn (Utilities|Struct|BreakEstructuraObjeto (.OutItem (Utilities|Array|Random (Variables|/Game/AuthenticationUI/OurGSGameMode.OurGSGameMode_C|GetObjetosSubnivel2_Strc _asour_gsgame_mode))))))) (Math|Random|RandomFloatinRange (.x (.RangoEscala (Utilities|Struct|BreakEstructuraObjeto (.OutItem (Utilities|Array|Random (Variables|/Game/AuthenticationUI/OurGSGameMode.OurGSGameMode_C|GetObjetosSubnivel2_Strc _asour_gsgame_mode)))))) (.y (.RangoEscala (Utilities|Struct|BreakEstructuraObjeto (.OutItem (Utilities|Array|Random (Variables|/Game/AuthenticationUI/OurGSGameMode.OurGSGameMode_C|GetObjetosSubnivel2_Strc _asour_gsgame_mode))))))) (.AmbosLados (Utilities|Struct|BreakEstructuraObjeto (.OutItem (Utilities|Array|Random (Variables|/Game/AuthenticationUI/OurGSGameMode.OurGSGameMode_C|GetObjetosSubnivel2_Strc _asour_gsgame_mode))))) (.Colores (Utilities|Struct|BreakEstructuraObjeto (.OutItem (Utilities|Array|Random (Variables|/Game/AuthenticationUI/OurGSGameMode.OurGSGameMode_C|GetObjetosSubnivel2_Strc _asour_gsgame_mode))))) (.AplicarShader (Utilities|Struct|BreakEstructuraObjeto (.OutItem (Utilities|Array|Random (Variables|/Game/AuthenticationUI/OurGSGameMode.OurGSGameMode_C|GetObjetosSubnivel2_Strc _asour_gsgame_mode))))))))))))
    (:then_1
      ;[1 1 1] Objetos Sub2 Bajada - Objetos Sub3 Subida
      (if (Variables|/Game/AuthenticationUI/OurGSGameMode.OurGSGameMode_C|GetObjetosSub2Bajada-ObjetosSub3Subida _asour_gsgame_mode)
        (for _array_element_2 (Variables|/Game/AuthenticationUI/OurGSGameMode.OurGSGameMode_C|GetObjetosSubnivel2_Strc _asour_gsgame_mode)
          (bind _aparicion__3 (CallFunction|ProbabilidadAparecimiento (Math|Float|Clamp(Float) (.NivelProbabilidad (Utilities|Struct|BreakEstructuraObjeto _array_element_2)) 0.0 (.ProbabilidadMaxima (Utilities|Struct|BreakEstructuraObjeto _array_element_2)))))
          (if _aparicion__3
            (ControlCasasObjetos()|GenerarObjetos (.Malla (Utilities|Struct|BreakEstructuraObjeto _array_element_2)) (Math|Random|RandomIntegerinRange (.x (.NumSpawn (Utilities|Struct|BreakEstructuraObjeto _array_element_2))) (.y (.NumSpawn (Utilities|Struct|BreakEstructuraObjeto _array_element_2)))) (Math|Random|RandomFloatinRange (.x (.RangoEscala (Utilities|Struct|BreakEstructuraObjeto _array_element_2))) (.y (.RangoEscala (Utilities|Struct|BreakEstructuraObjeto _array_element_2)))) (.AmbosLados (Utilities|Struct|BreakEstructuraObjeto _array_element_2)) (.Colores (Utilities|Struct|BreakEstructuraObjeto _array_element_2)) (.AplicarShader (Utilities|Struct|BreakEstructuraObjeto _array_element_2)))
            (else
              (bind _aparicion__4 (CallFunction|ProbabilidadAparecimiento (Math|Float|Clamp(Float) (.NivelProbabilidad (Utilities|Struct|BreakEstructuraObjeto (.OutItem (Utilities|Array|Random (Variables|/Game/AuthenticationUI/OurGSGameMode.OurGSGameMode_C|GetObjetosSubnivel3_Strc _asour_gsgame_mode))))) 0.0 (.ProbabilidadMaxima (Utilities|Struct|BreakEstructuraObjeto (.OutItem (Utilities|Array|Random (Variables|/Game/AuthenticationUI/OurGSGameMode.OurGSGameMode_C|GetObjetosSubnivel3_Strc _asour_gsgame_mode))))))))
              (if _aparicion__4
                (ControlCasasObjetos()|GenerarObjetos (.Malla (Utilities|Struct|BreakEstructuraObjeto (.OutItem (Utilities|Array|Random (Variables|/Game/AuthenticationUI/OurGSGameMode.OurGSGameMode_C|GetObjetosSubnivel3_Strc _asour_gsgame_mode))))) (Math|Random|RandomIntegerinRange (.x (.NumSpawn (Utilities|Struct|BreakEstructuraObjeto (.OutItem (Utilities|Array|Random (Variables|/Game/AuthenticationUI/OurGSGameMode.OurGSGameMode_C|GetObjetosSubnivel3_Strc _asour_gsgame_mode)))))) (.y (.NumSpawn (Utilities|Struct|BreakEstructuraObjeto (.OutItem (Utilities|Array|Random (Variables|/Game/AuthenticationUI/OurGSGameMode.OurGSGameMode_C|GetObjetosSubnivel3_Strc _asour_gsgame_mode))))))) (Math|Random|RandomFloatinRange (.x (.RangoEscala (Utilities|Struct|BreakEstructuraObjeto (.OutItem (Utilities|Array|Random (Variables|/Game/AuthenticationUI/OurGSGameMode.OurGSGameMode_C|GetObjetosSubnivel3_Strc _asour_gsgame_mode)))))) (.y (.RangoEscala (Utilities|Struct|BreakEstructuraObjeto (.OutItem (Utilities|Array|Random (Variables|/Game/AuthenticationUI/OurGSGameMode.OurGSGameMode_C|GetObjetosSubnivel3_Strc _asour_gsgame_mode))))))) (.AmbosLados (Utilities|Struct|BreakEstructuraObjeto (.OutItem (Utilities|Array|Random (Variables|/Game/AuthenticationUI/OurGSGameMode.OurGSGameMode_C|GetObjetosSubnivel3_Strc _asour_gsgame_mode))))) (.Colores (Utilities|Struct|BreakEstructuraObjeto (.OutItem (Utilities|Array|Random (Variables|/Game/AuthenticationUI/OurGSGameMode.OurGSGameMode_C|GetObjetosSubnivel3_Strc _asour_gsgame_mode))))) (.AplicarShader (Utilities|Struct|BreakEstructuraObjeto (.OutItem (Utilities|Array|Random (Variables|/Game/AuthenticationUI/OurGSGameMode.OurGSGameMode_C|GetObjetosSubnivel3_Strc _asour_gsgame_mode))))))))))))
    (:then_2
      ;[1 1 1] Objetos Sub3 Subida
      (if (Variables|/Game/AuthenticationUI/OurGSGameMode.OurGSGameMode_C|GetObjetosSub3_Subida _asour_gsgame_mode)
        (for _array_element_3 (Variables|/Game/AuthenticationUI/OurGSGameMode.OurGSGameMode_C|GetObjetosSubnivel3_Strc _asour_gsgame_mode)
          (bind _aparicion__5 (CallFunction|ProbabilidadAparecimiento (Math|Float|Clamp(Float) (.NivelProbabilidad (Utilities|Struct|BreakEstructuraObjeto _array_element_3)) 0.0 (.ProbabilidadMaxima (Utilities|Struct|BreakEstructuraObjeto _array_element_3)))))
          (if _aparicion__5
            (ControlCasasObjetos()|GenerarObjetos (.Malla (Utilities|Struct|BreakEstructuraObjeto _array_element_3)) (Math|Random|RandomIntegerinRange (.x (.NumSpawn (Utilities|Struct|BreakEstructuraObjeto _array_element_3))) (.y (.NumSpawn (Utilities|Struct|BreakEstructuraObjeto _array_element_3)))) (Math|Random|RandomFloatinRange (.x (.RangoEscala (Utilities|Struct|BreakEstructuraObjeto _array_element_3))) (.y (.RangoEscala (Utilities|Struct|BreakEstructuraObjeto _array_element_3)))) (.AmbosLados (Utilities|Struct|BreakEstructuraObjeto _array_element_3)) (.Colores (Utilities|Struct|BreakEstructuraObjeto _array_element_3)) (.AplicarShader (Utilities|Struct|BreakEstructuraObjeto _array_element_3)))))))
    (:then_3
      ;[1 1 1] Casas Sub1 a Sub2 a Sub3
      (if (Variables|/Game/AuthenticationUI/OurGSGameMode.OurGSGameMode_C|GetSubnivel2Cargado _asour_gsgame_mode)
        (bind _aparicion__6 (CallFunction|ProbabilidadAparecimiento (Variables|/Game/AuthenticationUI/OurGSGameMode.OurGSGameMode_C|GetProbabilidadSubnivel2 _asour_gsgame_mode))) ; Reducir casas sub 2
        (if _aparicion__6
          (ControlCasasObjetos()|GenerarEdificacionesSub2 (Variables|/Game/AuthenticationUI/OurGSGameMode.OurGSGameMode_C|GetArregloEdificiosSub2 _asour_gsgame_mode) (Variables|/Game/AuthenticationUI/OurGSGameMode.OurGSGameMode_C|GetArregloCasasSub2 _asour_gsgame_mode) :!label _label)
          (else
            (ControlCasasObjetos()|GenerarEdificacionesSub3 (Variables|/Game/AuthenticationUI/OurGSGameMode.OurGSGameMode_C|GetArregloEdificiosSub3 _asour_gsgame_mode) (Variables|/Game/AuthenticationUI/OurGSGameMode.OurGSGameMode_C|GetArregloCasasSub3 _asour_gsgame_mode))))
        (else
          (bind _aparicion__7 (CallFunction|ProbabilidadAparecimiento (Variables|/Game/AuthenticationUI/OurGSGameMode.OurGSGameMode_C|GetProbabilidadSubnivel1 _asour_gsgame_mode)))
          (if _aparicion__7
            (ControlCasasObjetos()|GenerarCasasSub1 (Variables|/Game/AuthenticationUI/OurGSGameMode.OurGSGameMode_C|GetCasasSubnivel1_Strc _asour_gsgame_mode))
            (else
              (goto _label))))))))

(fn SpawnDecalsSubnivel
  (params (ArregloDecals :type Array%20of%20Estructura%20Decal%20Structures))
  (bind _outitem (Utilities|Array|Random ArregloDecals))
  (bind _guiacentro (Variables|Default|GetGuiaCentro))
  (bind _returnvalue (Math|Random|RandomFloatinRange (.x (.sizerange _outitem)) (.y (.sizerange _outitem))))
  (bind _returnvalue_2 (Transformation|GetWorldLocation _guiacentro))
  (for _index (range 0 (Math|Random|RandomIntegerinRange (.x (.numspawn _outitem)) (.y (.numspawn _outitem))))
    (bind _aparicion_ (CallFunction|ProbabilidadAparecimiento (.probabilidad _outitem)))
    (if _aparicion_
      (Rendering|Decal|SpawnDecalatLocation (.decalmaterial _outitem) (Math|Vector|MakeVector 1e+02 _returnvalue _returnvalue) (Math|Vector|MakeVector (+ (Math|Random|RandomFloatinRange -2.5e+02 2.5e+02) (.x _returnvalue_2)) (+ (.y _returnvalue_2) (Math|Random|RandomFloatinRange -2.5e+02 2.5e+02)) (.z _returnvalue_2)) (Math|Rotator|MakeRotator 0.0 -9e+01 (Math|Random|RandomFloatinRange 0.0 3.6e+02)) 0.0))))

(fn SpawnDecals
  (bind _asour_gsgame_mode (Utilities|Casting|CastToOurGSGameMode (Game|GetGameMode)))
  (if (Variables|/Game/AuthenticationUI/OurGSGameMode.OurGSGameMode_C|GetSubnivel2Cargado _asour_gsgame_mode)
    (bind _aparicion_ (CallFunction|ProbabilidadAparecimiento (Variables|/Game/AuthenticationUI/OurGSGameMode.OurGSGameMode_C|GetProbabilidadSubnivel2 _asour_gsgame_mode)))
    (if _aparicion_
      (CallFunction|SpawnDecalsSubnivel (Variables|/Game/AuthenticationUI/OurGSGameMode.OurGSGameMode_C|GetDecalsSubnivel2 _asour_gsgame_mode) :!label _label)
      (else
        (CallFunction|SpawnDecalsSubnivel (Variables|/Game/AuthenticationUI/OurGSGameMode.OurGSGameMode_C|GetDecalsSubnivel3 _asour_gsgame_mode))))
    (else
      (bind _aparicion__2 (CallFunction|ProbabilidadAparecimiento (Variables|/Game/AuthenticationUI/OurGSGameMode.OurGSGameMode_C|GetProbabilidadSubnivel1 _asour_gsgame_mode)))
      (if _aparicion__2
        (CallFunction|SpawnDecalsSubnivel (Variables|/Game/AuthenticationUI/OurGSGameMode.OurGSGameMode_C|GetDecalsSubnivel1 _asour_gsgame_mode))
        (else
          (goto _label))))))

(fn SpawnObstaculosEstaticos
  (params (ActorObstaculo :type Obstaculo%20Sub%201%20BP%20Class%20Reference) (Fijar%20Posicion%20al%20Origen :type Boolean))
  (bind _guiacentro (Variables|Default|GetGuiaCentro))
  (bind _returnvalue (Transformation|GetWorldLocation _guiacentro))
  (if Fijar%20Posicion%20al%20Origen
    (bind _returnvalue_2 (Game|SpawnActorfromClass ActorObstaculo (Math|Transform|MakeTransform (Transformation|GetWorldLocation (Variables|Default|GetGuiaCentro)) "0, 0, 0" "1,1,1") "Undefined" 0 0))
    (Transformation|AttachActorToActor _returnvalue_2 self "None" "KeepWorld" "KeepRelative" "KeepRelative" true)
    (else
      (Game|SpawnActorfromClass ActorObstaculo (Math|Transform|MakeTransform (Math|Vector|MakeVector (+ (.x _returnvalue) (Math|Random|RandomFloatinRange -1e+02 1e+02)) (+ (.y _returnvalue) (Math|Random|RandomFloatinRange -1e+02 1e+02)) (.z _returnvalue)) "0, 0, 0" "1,1,1") "Undefined" 0 0))))

(fn ControlItems-Obstaculos
  (bind _asour_gsgame_mode (Utilities|Casting|CastToOurGSGameMode (Game|GetGameMode)))
  (Utilities|FlowControl|Sequence
    (:then_0
      (if (Variables|/Game/AuthenticationUI/OurGSGameMode.OurGSGameMode_C|GetActivarObstaculosEstaticosSub1 _asour_gsgame_mode)
        (bind _aparicion_ (CallFunction|ProbabilidadAparecimiento (Variables|/Game/AuthenticationUI/OurGSGameMode.OurGSGameMode_C|GetProb%20ObstaculosSub1 _asour_gsgame_mode)))
        (if _aparicion_
          (bind _aparicion__2 (CallFunction|ProbabilidadAparecimiento 0.5))
          (if _aparicion__2
            (CallFunction|SpawnObstaculosEstaticos "/Game/Runner_Files/Blueprints/Obstaculos/Clases/Obstaculo_sub1_BP.Obstaculo_sub1_BP_C" false)
            (else
              (CallFunction|SpawnObstaculosEstaticos "/Game/Runner_Files/Blueprints/Obstaculos/Clases/ObstaculoGrupo_sub1_BP.ObstaculoGrupo_sub1_BP_C" true))))))
    (:then_1
      (if (Variables|/Game/AuthenticationUI/OurGSGameMode.OurGSGameMode_C|GetActivarObstaculosEstaticosSub2 _asour_gsgame_mode)
        (bind _aparicion__3 (CallFunction|ProbabilidadAparecimiento (Variables|/Game/AuthenticationUI/OurGSGameMode.OurGSGameMode_C|GetProb%20ObstaculosSub2 _asour_gsgame_mode)))
        (if _aparicion__3
          (bind _aparicion__4 (CallFunction|ProbabilidadAparecimiento 0.5))
          (if _aparicion__4
            (CallFunction|SpawnObstaculosEstaticos "/Game/Runner_Files/Blueprints/Obstaculos/Clases/Obstaculo_sub2_BP.Obstaculo_sub2_BP_C" false)
            (else
              (CallFunction|SpawnObstaculosEstaticos "/Game/Runner_Files/Blueprints/Obstaculos/Clases/ObstaculoGrupo_sub2_BP.ObstaculoGrupo_sub2_BP_C" false))))))))

(fn GenerarCasasSub1
  (params (Arreglo :type Array%20of%20Estructura%20Casa%20Sub%201%20Structures))
  (bind _outitem (Utilities|Array|Random Arreglo))
  (bind (_malla _colores _aplicarshader) (Utilities|Struct|BreakEstructuraCasaSub1 _outitem))
  (for _index (range 0 6)
    (if (== _index 0)
      (LocalVariables|SetGuiaTemp (Variables|Default|GetGuia1CasaSub1))
      (bind _returnvalue (AddComponent|AddStaticMeshComponent false (Math|Transform|MakeTransform (.location (Transformation|GetRelativeTransform (LocalVariables|GetGuiaTemp))) (.rotation (Transformation|GetRelativeTransform (LocalVariables|GetGuiaTemp))) (.scale (Transformation|GetRelativeTransform (LocalVariables|GetGuiaTemp)))) :!label _label))
      (Rendering|SetRenderCustomDepth _returnvalue _aplicarshader)
      (bind _returnvalue_2 (Components|StaticMesh|SetStaticMesh _returnvalue _malla))
      (if _returnvalue_2
        (bind _returnvalue_3 (Rendering|Material|CreateDynamicMaterialInstance _returnvalue 0 (Rendering|Material|GetMaterial _returnvalue 0) "None" :!class /Script/Engine.PrimitiveComponent))
        (Rendering|Material|SetVectorParameterValue _returnvalue_3 "FactorColor" (Math|Conversions|ToLinearColor(Color) (Utilities|Array|Get(acopy) _colores (Math|Random|RandomIntegerinRange 0 (- (Utilities|Array|Length _colores) 1)))) :!class /Script/Engine.MaterialInstanceDynamic))
      (elif (== _index 1)
        (LocalVariables|SetGuiaTemp (Variables|Default|GetGuia2CasaSub1))
        (goto _label)
        (elif (== _index 2)
          (LocalVariables|SetGuiaTemp (Variables|Default|GetGuia3CasaSub1))
          (goto _label)
          (elif (== _index 3)
            (LocalVariables|SetGuiaTemp (Variables|Default|GetGuia4CasaSub1))
            (goto _label)
            (elif (== _index 4)
              (LocalVariables|SetGuiaTemp (Variables|Default|GetGuia5CasaSub1))
              (goto _label)
              (elif (== _index 5)
                (LocalVariables|SetGuiaTemp (Variables|Default|GetGuia6CasaSub1))
                (goto _label)
                (elif (== _index 6)
                  (LocalVariables|SetGuiaTemp (Variables|Default|GetGuia7CasaSub1))
                  (goto _label))))))))))

(fn GenerarEdificacionesSub2
  (params (ArregloEdificios :type Array%20of%20Estructura%20Casa%20Sub%202%20Structures) (ArregloCasas :type Array%20of%20Estructura%20Casa%20Sub%202%20Structures))
  (if (or (== (Utilities|Array|Length ArregloEdificios) 0) (== (Utilities|Array|Length ArregloCasas) 0))
    (Development|PrintString "ALERTA!   Arreclo Casas Sub2  " true true "(R=1.000000,G=0.013449,B=0.000000,A=1.000000)" 5.0)
    (else
      (ControlCasasObjetos()|GenerarCasasSub2 ArregloCasas)
      (ControlCasasObjetos()|GenerarEdificiosSub2 ArregloEdificios))))

(fn GenerarCasasSub2
  (params (ArregloCasas :type Array%20of%20Estructura%20Casa%20Sub%202%20Structures))
  (bind _outitem (Utilities|Array|Random ArregloCasas))
  (bind _giro_0_180 (LocalVariables|GetGiro_0_180))
  (bind _giro_0_180_2 (LocalVariables|GetGiro_0_180))
  (bind (_espaciousado _malla _colores _aplicarshader _giro_0_180_3) (Utilities|Struct|BreakEstructuraCasaSub2 _outitem))
  (for _index (range 1 4)
    (if (== _index 1)
      (LocalVariables|SetGuia_Temp (Variables|Default|GetGuia1CasaSub2Sub3))
      (if _giro_0_180_3 :!label _label
        (Utilities|Array|SetArrayElem _giro_0_180_2 0 0)
        (Utilities|Array|SetArrayElem _giro_0_180_2 1 180)
        (else
          (Utilities|Array|SetArrayElem _giro_0_180 0 0)
          (Utilities|Array|SetArrayElem _giro_0_180 1 0)))
      (bind _returnvalue (AddComponent|AddStaticMeshComponent false (Math|Transform|MakeTransform (.location (Transformation|GetRelativeTransform (LocalVariables|GetGuia_Temp))) (Math|Rotator|MakeRotator 0.0 0.0 (Math|Conversions|ToFloat(Integer) (.OutItem (Utilities|Array|Random (LocalVariables|GetGiro_0_180))))) (.scale (Transformation|GetRelativeTransform (LocalVariables|GetGuia_Temp))))))
      (Rendering|SetRenderCustomDepth _returnvalue _aplicarshader)
      (bind _returnvalue_2 (Components|StaticMesh|SetStaticMesh _returnvalue _malla))
      (if _returnvalue_2
        (bind _returnvalue_3 (Rendering|Material|CreateDynamicMaterialInstance _returnvalue 0 (Rendering|Material|GetMaterial _returnvalue 0) "None" :!class /Script/Engine.PrimitiveComponent))
        (Rendering|Material|SetVectorParameterValue _returnvalue_3 "FactorColor" (Math|Conversions|ToLinearColor(Color) (Utilities|Array|Get(acopy) _colores (Math|Random|RandomIntegerinRange 0 (- (Utilities|Array|Length _colores) 1)))) :!class /Script/Engine.MaterialInstanceDynamic))
      (elif (== _index 2)
        (LocalVariables|SetGuia_Temp (Variables|Default|GetGuia2CasaSub2Sub3))
        (goto _label)
        (elif (== _index 3)
          (LocalVariables|SetGuia_Temp (Variables|Default|GetGuia3CasaSub2Sub3))
          (goto _label)
          (elif (== _index 4)
            (LocalVariables|SetGuia_Temp (Variables|Default|GetGuia4CasaSub2Sub3))
            (goto _label)))))))

(fn GenerarEdificiosSub2
  (params (ArregloEdificios :type Array%20of%20Estructura%20Casa%20Sub%202%20Structures))
  (bind _outitem (Utilities|Array|Random ArregloEdificios))
  (bind (_espaciousado _malla _colores _aplicarshader) (Utilities|Struct|BreakEstructuraCasaSub2 _outitem))
  (for _index (range 0 4)
    (if (== _index 0)
      (LocalVariables|SetGuia_Temp (Variables|Default|GetGuia5CasaSub2Sub3))
      (bind _returnvalue (AddComponent|AddStaticMeshComponent false (Transformation|GetRelativeTransform (LocalVariables|GetGuia_Temp)) :!label _label))
      (Rendering|SetRenderCustomDepth _returnvalue _aplicarshader)
      (bind _returnvalue_2 (Components|StaticMesh|SetStaticMesh _returnvalue _malla))
      (if _returnvalue_2
        (bind _returnvalue_3 (Rendering|Material|CreateDynamicMaterialInstance _returnvalue 0 (Rendering|Material|GetMaterial _returnvalue 0) "None" :!class /Script/Engine.PrimitiveComponent))
        (Rendering|Material|SetVectorParameterValue _returnvalue_3 "FactorColor" (Math|Conversions|ToLinearColor(Color) (Utilities|Array|Get(acopy) _colores (Math|Random|RandomIntegerinRange 0 (- (Utilities|Array|Length _colores) 1)))) :!class /Script/Engine.MaterialInstanceDynamic))
      (elif (== _index 1)
        (LocalVariables|SetGuia_Temp (Variables|Default|GetGuia6CasaSub2Sub3))
        (goto _label)
        (elif (== _index 2)
          (LocalVariables|SetGuia_Temp (Variables|Default|GetGuia7CasaSub2Sub3))
          (goto _label)
          (elif (== _index 3)
            (LocalVariables|SetGuia_Temp (Variables|Default|GetGuia8CasaSub2Sub3))
            (goto _label)
            (elif (== _index 4)
              (LocalVariables|SetGuia_Temp (Variables|Default|GetGuia9CasaSub2Sub3))
              (goto _label))))))))

(fn GenerarEdificacionesSub3
  (params (ArregloEdificios :type Array%20of%20Estructura%20Casa%20Sub%203%20Structures) (ArregloCasas :type Array%20of%20Estructura%20Casa%20Sub%203%20Structures))
  (if (or (== (Utilities|Array|Length ArregloEdificios) 0) (== (Utilities|Array|Length ArregloCasas) 0))
    (Development|PrintString "ALERTA!   Arreclo Casas Sub3" true true "(R=1.000000,G=0.013449,B=0.000000,A=1.000000)" 5.0)
    (else
      (ControlCasasObjetos()|GenerarCasasSub3 ArregloCasas)
      (ControlCasasObjetos()|GenerarEdificiosSub3 ArregloEdificios))))

(fn GenerarCasasSub3
  (params (ArregloCasas :type Array%20of%20Estructura%20Casa%20Sub%203%20Structures))
  (bind _outitem (Utilities|Array|Random ArregloCasas))
  (bind _giro_0_180 (LocalVariables|GetGiro_0_180))
  (bind _giro_0_180_2 (LocalVariables|GetGiro_0_180))
  (bind (_espaciousado _actor _colores _aplicarshader _giro_0_180_3) (Utilities|Struct|BreakEstructuraCasaSub3 _outitem))
  (for _index (range 1 4)
    (if (== _index 1)
      (LocalVariables|SetGuia_Temp (Variables|Default|GetGuia1CasaSub2Sub3))
      (if _giro_0_180_3 :!label _label
        (Utilities|Array|SetArrayElem _giro_0_180 0 0)
        (Utilities|Array|SetArrayElem _giro_0_180 1 180)
        (else
          (Utilities|Array|SetArrayElem _giro_0_180_2 0 0)
          (Utilities|Array|SetArrayElem _giro_0_180_2 1 0)))
      (bind _returnvalue (Game|SpawnActorfromClass _actor (Math|Transform|MakeTransform (.location (Transformation|GetRelativeTransform (LocalVariables|GetGuia_Temp))) (Math|Rotator|MakeRotator 0.0 0.0 (Math|Conversions|ToFloat(Integer) (.OutItem (Utilities|Array|Random (LocalVariables|GetGiro_0_180))))) (.scale (Transformation|GetRelativeTransform (LocalVariables|GetGuia_Temp)))) "Undefined" 0 0))
      (Rendering|SetRenderCustomDepth (Variables|/Game/Runner_Files/Meshes/Merged/Level_3/Actors/Casa_MASTER_n3_01.Casa_MASTER_n3_01_C|Getcasa _returnvalue) _aplicarshader)
      (Transformation|AttachActorToActor _returnvalue self "None" "KeepRelative" "KeepRelative" "KeepRelative" true)
      (elif (== _index 2)
        (LocalVariables|SetGuia_Temp (Variables|Default|GetGuia2CasaSub2Sub3))
        (goto _label)
        (elif (== _index 3)
          (LocalVariables|SetGuia_Temp (Variables|Default|GetGuia3CasaSub2Sub3))
          (goto _label)
          (elif (== _index 4)
            (LocalVariables|SetGuia_Temp (Variables|Default|GetGuia4CasaSub2Sub3))
            (goto _label)))))))

(fn GenerarEdificiosSub3
  (params (ArregloEdificios :type Array%20of%20Estructura%20Casa%20Sub%203%20Structures))
  (bind _outitem (Utilities|Array|Random ArregloEdificios))
  (bind (_espaciousado _actor _colores _aplicarshader) (Utilities|Struct|BreakEstructuraCasaSub3 _outitem))
  (for _index (range 1 4)
    (if (== _index 1)
      (LocalVariables|SetGuia_Temp (Variables|Default|GetGuia5CasaSub2Sub3))
      (bind _returnvalue (Game|SpawnActorfromClass _actor (Transformation|GetRelativeTransform (LocalVariables|GetGuia_Temp)) "Undefined" 0 0 :!label _label))
      (Rendering|SetRenderCustomDepth (Variables|/Game/Runner_Files/Meshes/Merged/Level_3/Actors/Casa_MASTER_n3_01.Casa_MASTER_n3_01_C|Getcasa _returnvalue) _aplicarshader)
      (Transformation|AttachActorToActor _returnvalue self "None" "KeepRelative" "KeepRelative" "KeepRelative" true)
      (elif (== _index 2)
        (LocalVariables|SetGuia_Temp (Variables|Default|GetGuia6CasaSub2Sub3))
        (goto _label)
        (elif (== _index 3)
          (LocalVariables|SetGuia_Temp (Variables|Default|GetGuia7CasaSub2Sub3))
          (goto _label)
          (elif (== _index 4)
            (LocalVariables|SetGuia_Temp (Variables|Default|GetGuia8CasaSub2Sub3))
            (goto _label)
            (elif (== _index 5)
              (LocalVariables|SetGuia_Temp (Variables|Default|GetGuia9CasaSub2Sub3))
              (goto _label))))))))