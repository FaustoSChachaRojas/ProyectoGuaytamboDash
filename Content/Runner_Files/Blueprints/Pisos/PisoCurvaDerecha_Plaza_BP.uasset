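; Right-turn plaza floor tile for an endless runner that sets the game mode's next spawn point and turn direction on BeginPlay.
; It offsets the floor material and scatters houses, props and decals at guide components, using sublevel-driven probabilities from game mode arrays, with random tints on meshes.
; Overlap triggers play the character's turn animation and spawn the next tile.
; Tick destroys the tile after a delay once the player has left.
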(event OnComponentBeginOverlap(BoxCollision_Animacion)
  (params (OverlappedComponent :type Primitive%20Component%20Object%20Reference) (OtherActor :type Actor%20Object%20Reference) (OtherComp :type Primitive%20Component%20Object%20Reference) (OtherBodyIndex :type Integer) (bFromSweep :type Boolean) (SweepResult :type Hit%20Result%20Structure%20%28by%20ref%29))
  (bind _asrun_character (Utilities|Casting|CastToRunCharacter OtherActor))
  (Default|AnimacionGiroDerecho _asrun_character)
  (bind _asour_gsgame_mode (Utilities|Casting|CastToOurGSGameMode (Game|GetGameMode)))
  (Default|SpawnTile _asour_gsgame_mode))

(event OnComponentBeginOverlap(Estadia)
  (params (OverlappedComponent :type Primitive%20Component%20Object%20Reference) (OtherActor :type Actor%20Object%20Reference) (OtherComp :type Primitive%20Component%20Object%20Reference) (OtherBodyIndex :type Integer) (bFromSweep :type Boolean) (SweepResult :type Hit%20Result%20Structure%20%28by%20ref%29))
  (Utilities|Casting|CastToRunCharacter OtherActor)
  (Variables|Default|SetEntroPersonaje true))

(event EventBeginPlay
  (Utilities|FlowControl|Sequence
    (:then_0
      (CallFunction|OffsetMaterialPisoMaster)
      (CallFunction|FijarPosicionSpawn))
    (:then_1
      (ControlCasasObjetos()|ControlCasasObjetos))
    (:then_2
      (CallFunction|SpawnDecals))))

(event EventTick
  (params (DeltaSeconds :type Float%20%28single-precision%29))
  (bind _asrun_character (Utilities|Casting|CastToRunCharacter (Game|Player|GetPlayerPawn 0)))
  (if (not (Collision|IsOverlappingActor (Variables|Default|GetEstadia) _asrun_character :!class /Script/Engine.PrimitiveComponent))
    (if (Variables|Default|GetEntroPersonaje)
      (Utilities|FlowControl|Delay 2.0)
      (Actor|DestroyActor))))

(fn ConstructionScript)

(fn FijarPosicionSpawn
  (bind _puntoaparecercd (Variables|Default|GetPuntoAparecerCD))
  (bind _asour_gsgame_mode (Utilities|Casting|CastToOurGSGameMode (Game|GetGameMode)))
  (bind _output_get (Variables|/Game/AuthenticationUI/OurGSGameMode.OurGSGameMode_C|SetDireccionGiro _asour_gsgame_mode (Math|Rotator|MakeRotator 0.0 0.0 (Math|Conversions|ToFloat(Integer) (Math|Float|Round (.Yaw (Math|Rotator|BreakRotator (Transformation|GetWorldRotation _puntoaparecercd))))))))
  (Variables|/Game/AuthenticationUI/OurGSGameMode.OurGSGameMode_C|SetNextSpawnPoint _asour_gsgame_mode (Math|Transform|MakeTransform (Transformation|GetWorldLocation _puntoaparecercd) _output_get "1,1,1"))
  (bind _asrun_character (Utilities|Casting|CastToRunCharacter (Game|GetPlayerCharacter 0)))
  (Variables|/Game/RunnerPersonBP/Blueprints/RunCharacter.RunCharacter_C|SetCambiarPisoCurvoDerecha _asrun_character false))

(fn GenerarCasas
  (params (Espacios :type SizeMesh_Enum%20Enum :default "NewEnumerator4") (Malla :type Static%20Mesh%20Object%20Reference) (Colores :type Array%20of%20Color%20Structures) (AplicarShader :type Boolean))
  (bind _returnvalue (Utilities|Array|Length Colores))
  (bind _returnvalue_2 (- _returnvalue 1))
  (bind _returnvalue_3 (Math|Random|RandomIntegerinRange 0 _returnvalue_2))
  (bind _output (Utilities|Array|Get(acopy) Colores _returnvalue_3))
  (bind _returnvalue_4 (Math|Conversions|ToLinearColor(Color) _output))
  (if (Utilities|Enum|Equal(Enum) Espacios "NewEnumerator4")
    (for _index (range 0 3)
      (if (== _index 0)
        (Variables|Script|SetGuiaTemp_CasasRuinas (Variables|Default|GetGuia1Casa))
        (bind _returnvalue_5 (AddComponent|AddStaticMeshComponent false (Math|Transform|MakeTransform (.location (Transformation|GetRelativeTransform (Variables|Script|GetGuiaTemp_CasasRuinas))) (Math|Rotator|MakeRotator 0.0 0.0 (Math|Conversions|ToFloat(Integer) (Utilities|Array|Get(acopy) (Variables|Script|GetGirosPerpendiculares_CasasRuinas) (Math|Random|RandomIntegerinRange 0 3)))) (.scale (Transformation|GetRelativeTransform (Variables|Script|GetGuiaTemp_CasasRuinas)))) :!label _label))
        (Rendering|SetRenderCustomDepth _returnvalue_5 AplicarShader)
        (bind _returnvalue_6 (Components|StaticMesh|SetStaticMesh _returnvalue_5 Malla))
        (if _returnvalue_6
          (bind _returnvalue_7 (Rendering|Material|CreateDynamicMaterialInstance _returnvalue_5 0 (Rendering|Material|GetMaterial _returnvalue_5 0) "None" :!class /Script/Engine.PrimitiveComponent))
          (Rendering|Material|SetVectorParameterValue _returnvalue_7 "FactorColor" _returnvalue_4 :!class /Script/Engine.MaterialInstanceDynamic))
        (elif (== _index 1)
          (Variables|Script|SetGuiaTemp_CasasRuinas (Variables|Default|GetGuia2Casa))
          (goto _label)
          (elif (== _index 2)
            (Variables|Script|SetGuiaTemp_CasasRuinas (Variables|Default|GetGuia3Casa))
            (goto _label)
            (elif (== _index 3)
              (Variables|Script|SetGuiaTemp_CasasRuinas (Variables|Default|GetGuia4Casa))
              (goto _label))))))
    (elif (Utilities|Enum|Equal(Enum) Espacios "NewEnumerator0")
      (for _index_2 (range 0 3)
        (if (== _index_2 0)
          (Variables|Script|SetGuiaTemp_CasasRuinas (Variables|Default|GetGuia1CasaSub2))
          (bind _returnvalue_8 (AddComponent|AddStaticMeshComponent false (Math|Transform|MakeTransform (.location (Transformation|GetRelativeTransform (Variables|Script|GetGuiaTemp_CasasRuinas))) (.rotation (Transformation|GetRelativeTransform (Variables|Script|GetGuiaTemp_CasasRuinas))) (.scale (Transformation|GetRelativeTransform (Variables|Script|GetGuiaTemp_CasasRuinas)))) :!label _label_2))
          (Rendering|SetRenderCustomDepth _returnvalue_8 AplicarShader)
          (bind _returnvalue_9 (Components|StaticMesh|SetStaticMesh _returnvalue_8 Malla))
          (if _returnvalue_9
            (bind _returnvalue_10 (Rendering|Material|CreateDynamicMaterialInstance _returnvalue_8 0 (Rendering|Material|GetMaterial _returnvalue_8 0) "None" :!class /Script/Engine.PrimitiveComponent))
            (Rendering|Material|SetVectorParameterValue _returnvalue_10 "FactorColor" _returnvalue_4 :!class /Script/Engine.MaterialInstanceDynamic))
          (elif (== _index_2 1)
            (Variables|Script|SetGuiaTemp_CasasRuinas (Variables|Default|GetGuia2CasaSub2))
            (goto _label_2)
            (elif (== _index_2 2)
              (Variables|Script|SetGuiaTemp_CasasRuinas (Variables|Default|GetGuia3CasaSub2))
              (goto _label_2)
              (elif (== _index_2 3)
                (Variables|Script|SetGuiaTemp_CasasRuinas (Variables|Default|GetGuia4CasaSub2))
                (goto _label_2)))))))))

(fn GenerarObjetos
  (params (Malla :type Static%20Mesh%20Object%20Reference) (NumSpawn :type Integer) (Escala :type Float%20%28single-precision%29) (AmbosLados :type Boolean) (Distancia_Spawn_Izq :type Float%20%28single-precision%29) (Distancia_Spawn_Der :type Float%20%28single-precision%29) (Colores :type Array%20of%20Color%20Structures) (AplicarShader :type Boolean))
  (for _index (range 0 2) ; Se escoge cada guia
    (if (== _index 0)
      (Variables|Script|SetGuiaTemp_Escombros (Variables|Default|GetGuiaObjetos1))
      (Variables|Script|SetIndiceDistanciasGuias 0)
      (for _index_2 (range 1 NumSpawn) :!label _label ; POr cada guia se spawnea 4 veces
        (bind _returnvalue (AddComponent|AddStaticMeshComponent false (Math|Transform|MakeTransform (Math|Vector|MakeVector (+ (Math|Random|RandomFloatinRange (.x (Utilities|Array|Get(acopy) (Variables|Script|GetDistanciasGuias) (Variables|Script|GetIndiceDistanciasGuias))) (.y (Utilities|Array|Get(acopy) (Variables|Script|GetDistanciasGuias) (Variables|Script|GetIndiceDistanciasGuias)))) (.x (.location (Transformation|GetRelativeTransform (Variables|Script|GetGuiaTemp_Escombros))))) (+ (Math|Random|RandomFloatinRange (.z (Utilities|Array|Get(acopy) (Variables|Script|GetDistanciasGuias) (Variables|Script|GetIndiceDistanciasGuias))) (.w (Utilities|Array|Get(acopy) (Variables|Script|GetDistanciasGuias) (Variables|Script|GetIndiceDistanciasGuias)))) (.y (.location (Transformation|GetRelativeTransform (Variables|Script|GetGuiaTemp_Escombros))))) 0.0) (Math|Rotator|MakeRotator 0.0 0.0 (Math|Random|RandomFloatinRange 0.0 3.6e+02)) (Math|Vector|MakeVector Escala Escala Escala))))
        (Rendering|SetRenderCustomDepth _returnvalue AplicarShader)
        (Components|StaticMesh|SetStaticMesh _returnvalue Malla)
        (bind _returnvalue_2 (Rendering|Material|CreateDynamicMaterialInstance _returnvalue 0 (Rendering|Material|GetMaterial _returnvalue 0) "None" :!class /Script/Engine.PrimitiveComponent))
        (Rendering|Material|SetVectorParameterValue _returnvalue_2 "FactorColor" (Math|Conversions|ToLinearColor(Color) (Utilities|Array|Get(acopy) Colores (Math|Random|RandomIntegerinRange 0 (- (Utilities|Array|Length Colores) 1)))) :!class /Script/Engine.MaterialInstanceDynamic) ; se cambia el color de las mallas
      )
      (elif (== _index 1)
        (Variables|Script|SetGuiaTemp_Escombros (Variables|Default|GetGuiaObjetos2))
        (Variables|Script|SetIndiceDistanciasGuias 1)
        (goto _label)
        (elif (== _index 2)
          (Variables|Script|SetGuiaTemp_Escombros (Variables|Default|GetGuiaObjetos3))
          (Variables|Script|SetIndiceDistanciasGuias 2)
          (goto _label))))))

(fn ProbabilidadAparecimiento
  (params (NivelProbabildiad :type Float%20%28single-precision%29))
  (return (Math|Float|InRange(Float) (Math|Random|RandomFloatinRange 0.0 1.0) 0.0 NivelProbabildiad)))

(fn OffsetMaterialPisoMaster
  (bind _pisocurvo (Variables|Default|GetPisoCurvo))
  (bind _returnvalue (Rendering|Material|CreateDynamicMaterialInstance _pisocurvo 0 (Rendering|Material|GetMaterial _pisocurvo 0) "None" :!class /Script/Engine.PrimitiveComponent))
  (Rendering|Material|SetVectorParameterValue _returnvalue "DesplazamientoUV" (Utilities|Struct|MakeLinearColor (Math|Random|RandomFloatinRange 0.0 1.0) 0.0 0.0 1.0) :!class /Script/Engine.MaterialInstanceDynamic)
  (bind _asour_gsgame_mode (Utilities|Casting|CastToOurGSGameMode (Game|GetGameMode)))
  (Rendering|Material|SetScalarParameterValue _returnvalue "Interpolacion" (Variables|/Game/AuthenticationUI/OurGSGameMode.OurGSGameMode_C|GetScalarParameterMaterial_Tiles _asour_gsgame_mode) :!class /Script/Engine.MaterialInstanceDynamic))

(fn ControlCasasObjetos
  (bind _asour_gsgame_mode (Utilities|Casting|CastToOurGSGameMode (Game|GetGameMode)))
  (Utilities|FlowControl|Sequence
    (:then_0
      ;[1 1 1] ObjetosSub1Bajada-ObjetosSub2Subida
      (if (Variables|/Game/AuthenticationUI/OurGSGameMode.OurGSGameMode_C|GetObjetosSub1_Bajada-ObjetosSub2_Subida _asour_gsgame_mode)
        (for _array_element (Variables|/Game/AuthenticationUI/OurGSGameMode.OurGSGameMode_C|GetObjetosSubnivel1_Strc _asour_gsgame_mode)
          (bind _aparicion_ (CallFunction|ProbabilidadAparecimiento (Math|Float|Clamp(Float) (.NivelProbabilidad (Utilities|Struct|BreakEstructuraObjeto _array_element)) 0.0 (.ProbabilidadMaxima (Utilities|Struct|BreakEstructuraObjeto _array_element)))))
          (if _aparicion_
            (ControlCasasObjetos()|GenerarObjetos (.Malla (Utilities|Struct|BreakEstructuraObjeto _array_element)) (Math|Random|RandomIntegerinRange (.x (.NumSpawn (Utilities|Struct|BreakEstructuraObjeto _array_element))) (.y (.NumSpawn (Utilities|Struct|BreakEstructuraObjeto _array_element)))) (Math|Random|RandomFloatinRange (.x (.RangoEscala (Utilities|Struct|BreakEstructuraObjeto _array_element))) (.y (.RangoEscala (Utilities|Struct|BreakEstructuraObjeto _array_element)))) (.AmbosLados (Utilities|Struct|BreakEstructuraObjeto _array_element)) (.x (.Distancia_Spawn (Utilities|Struct|BreakEstructuraObjeto _array_element))) (.y (.Distancia_Spawn (Utilities|Struct|BreakEstructuraObjeto _array_element))) (.Colores (Utilities|Struct|BreakEstructuraObjeto _array_element)) (.AplicarShader (Utilities|Struct|BreakEstructuraObjeto _array_element)))
            (else
              (bind _aparicion__2 (CallFunction|ProbabilidadAparecimiento (Math|Float|Clamp(Float) (.nivelprobabilidad (.OutItem (Utilities|Array|Random (Variables|/Game/AuthenticationUI/OurGSGameMode.OurGSGameMode_C|GetObjetosSubnivel2_Strc _asour_gsgame_mode)))) 0.0 (.probabilidadmaxima (.OutItem (Utilities|Array|Random (Variables|/Game/AuthenticationUI/OurGSGameMode.OurGSGameMode_C|GetObjetosSubnivel2_Strc _asour_gsgame_mode)))))))
              (if _aparicion__2
                (ControlCasasObjetos()|GenerarObjetos (.malla (.OutItem (Utilities|Array|Random (Variables|/Game/AuthenticationUI/OurGSGameMode.OurGSGameMode_C|GetObjetosSubnivel2_Strc _asour_gsgame_mode)))) (Math|Random|RandomIntegerinRange (.x (.numspawn (.OutItem (Utilities|Array|Random (Variables|/Game/AuthenticationUI/OurGSGameMode.OurGSGameMode_C|GetObjetosSubnivel2_Strc _asour_gsgame_mode))))) (.y (.numspawn (.OutItem (Utilities|Array|Random (Variables|/Game/AuthenticationUI/OurGSGameMode.OurGSGameMode_C|GetObjetosSubnivel2_Strc _asour_gsgame_mode)))))) (Math|Random|RandomFloatinRange (.x (.rangoescala (.OutItem (Utilities|Array|Random (Variables|/Game/AuthenticationUI/OurGSGameMode.OurGSGameMode_C|GetObjetosSubnivel2_Strc _asour_gsgame_mode))))) (.y (.rangoescala (.OutItem (Utilities|Array|Random (Variables|/Game/AuthenticationUI/OurGSGameMode.OurGSGameMode_C|GetObjetosSubnivel2_Strc _asour_gsgame_mode)))))) (.amboslados (.OutItem (Utilities|Array|Random (Variables|/Game/AuthenticationUI/OurGSGameMode.OurGSGameMode_C|GetObjetosSubnivel2_Strc _asour_gsgame_mode)))) (.x (.distancia_spawn (.OutItem (Utilities|Array|Random (Variables|/Game/AuthenticationUI/OurGSGameMode.OurGSGameMode_C|GetObjetosSubnivel2_Strc _asour_gsgame_mode))))) (.y (.distancia_spawn (.OutItem (Utilities|Array|Random (Variables|/Game/AuthenticationUI/OurGSGameMode.OurGSGameMode_C|GetObjetosSubnivel2_Strc _asour_gsgame_mode))))) (.colores (.OutItem (Utilities|Array|Random (Variables|/Game/AuthenticationUI/OurGSGameMode.OurGSGameMode_C|GetObjetosSubnivel2_Strc _asour_gsgame_mode)))) (.aplicarshader (.OutItem (Utilities|Array|Random (Variables|/Game/AuthenticationUI/OurGSGameMode.OurGSGameMode_C|GetObjetosSubnivel2_Strc _asour_gsgame_mode)))))))))))
    (:then_1
      ;[1 1 1] Objetos Sub2 Bajada - Objetos Sub3 Subida
      (if (Variables|/Game/AuthenticationUI/OurGSGameMode.OurGSGameMode_C|GetObjetosSub2Bajada-ObjetosSub3Subida _asour_gsgame_mode)
        (for _array_element_2 (Variables|/Game/AuthenticationUI/OurGSGameMode.OurGSGameMode_C|GetObjetosSubnivel2_Strc _asour_gsgame_mode)
          (bind _aparicion__3 (CallFunction|ProbabilidadAparecimiento (Math|Float|Clamp(Float) (.NivelProbabilidad (Utilities|Struct|BreakEstructuraObjeto _array_element_2)) 0.0 (.ProbabilidadMaxima (Utilities|Struct|BreakEstructuraObjeto _array_element_2)))))
          (if _aparicion__3
            (ControlCasasObjetos()|GenerarObjetos (.Malla (Utilities|Struct|BreakEstructuraObjeto _array_element_2)) (Math|Random|RandomIntegerinRange (.x (.NumSpawn (Utilities|Struct|BreakEstructuraObjeto _array_element_2))) (.y (.NumSpawn (Utilities|Struct|BreakEstructuraObjeto _array_element_2)))) (Math|Random|RandomFloatinRange (.x (.RangoEscala (Utilities|Struct|BreakEstructuraObjeto _array_element_2))) (.y (.RangoEscala (Utilities|Struct|BreakEstructuraObjeto _array_element_2)))) (.AmbosLados (Utilities|Struct|BreakEstructuraObjeto _array_element_2)) (.x (.Distancia_Spawn (Utilities|Struct|BreakEstructuraObjeto _array_element_2))) (.y (.Distancia_Spawn (Utilities|Struct|BreakEstructuraObjeto _array_element_2))) (.Colores (Utilities|Struct|BreakEstructuraObjeto _array_element_2)) (.AplicarShader (Utilities|Struct|BreakEstructuraObjeto _array_element_2)))
            (else
              (bind _aparicion__4 (CallFunction|ProbabilidadAparecimiento (Math|Float|Clamp(Float) (.nivelprobabilidad (.OutItem (Utilities|Array|Random (Variables|/Game/AuthenticationUI/OurGSGameMode.OurGSGameMode_C|GetObjetosSubnivel3_Strc _asour_gsgame_mode)))) 0.0 (.probabilidadmaxima (.OutItem (Utilities|Array|Random (Variables|/Game/AuthenticationUI/OurGSGameMode.OurGSGameMode_C|GetObjetosSubnivel3_Strc _asour_gsgame_mode)))))))
              (if _aparicion__4
                (ControlCasasObjetos()|GenerarObjetos (.malla (.OutItem (Utilities|Array|Random (Variables|/Game/AuthenticationUI/OurGSGameMode.OurGSGameMode_C|GetObjetosSubnivel3_Strc _asour_gsgame_mode)))) (Math|Random|RandomIntegerinRange (.x (.numspawn (.OutItem (Utilities|Array|Random (Variables|/Game/AuthenticationUI/OurGSGameMode.OurGSGameMode_C|GetObjetosSubnivel3_Strc _asour_gsgame_mode))))) (.y (.numspawn (.OutItem (Utilities|Array|Random (Variables|/Game/AuthenticationUI/OurGSGameMode.OurGSGameMode_C|GetObjetosSubnivel3_Strc _asour_gsgame_mode)))))) (Math|Random|RandomFloatinRange (.x (.rangoescala (.OutItem (Utilities|Array|Random (Variables|/Game/AuthenticationUI/OurGSGameMode.OurGSGameMode_C|GetObjetosSubnivel3_Strc _asour_gsgame_mode))))) (.y (.rangoescala (.OutItem (Utilities|Array|Random (Variables|/Game/AuthenticationUI/OurGSGameMode.OurGSGameMode_C|GetObjetosSubnivel3_Strc _asour_gsgame_mode)))))) (.amboslados (.OutItem (Utilities|Array|Random (Variables|/Game/AuthenticationUI/OurGSGameMode.OurGSGameMode_C|GetObjetosSubnivel3_Strc _asour_gsgame_mode)))) (.x (.distancia_spawn (.OutItem (Utilities|Array|Random (Variables|/Game/AuthenticationUI/OurGSGameMode.OurGSGameMode_C|GetObjetosSubnivel3_Strc _asour_gsgame_mode))))) (.y (.distancia_spawn (.OutItem (Utilities|Array|Random (Variables|/Game/AuthenticationUI/OurGSGameMode.OurGSGameMode_C|GetObjetosSubnivel3_Strc _asour_gsgame_mode))))) (.colores (.OutItem (Utilities|Array|Random (Variables|/Game/AuthenticationUI/OurGSGameMode.OurGSGameMode_C|GetObjetosSubnivel3_Strc _asour_gsgame_mode)))) (.aplicarshader (.OutItem (Utilities|Array|Random (Variables|/Game/AuthenticationUI/OurGSGameMode.OurGSGameMode_C|GetObjetosSubnivel3_Strc _asour_gsgame_mode)))))))))))
    (:then_2
      ;[1 1 1] Objetos Sub3 Subida
      (if (Variables|/Game/AuthenticationUI/OurGSGameMode.OurGSGameMode_C|GetObjetosSub3_Subida _asour_gsgame_mode)
        (for _array_element_3 (Variables|/Game/AuthenticationUI/OurGSGameMode.OurGSGameMode_C|GetObjetosSubnivel3_Strc _asour_gsgame_mode)
          (bind _aparicion__5 (CallFunction|ProbabilidadAparecimiento (Math|Float|Clamp(Float) (.NivelProbabilidad (Utilities|Struct|BreakEstructuraObjeto _array_element_3)) 0.0 (.ProbabilidadMaxima (Utilities|Struct|BreakEstructuraObjeto _array_element_3)))))
          (if _aparicion__5
            (ControlCasasObjetos()|GenerarObjetos (.Malla (Utilities|Struct|BreakEstructuraObjeto _array_element_3)) (Math|Random|RandomIntegerinRange (.x (.NumSpawn (Utilities|Struct|BreakEstructuraObjeto _array_element_3))) (.y (.NumSpawn (Utilities|Struct|BreakEstructuraObjeto _array_element_3)))) (Math|Random|RandomFloatinRange (.x (.RangoEscala (Utilities|Struct|BreakEstructuraObjeto _array_element_3))) (.y (.RangoEscala (Utilities|Struct|BreakEstructuraObjeto _array_element_3)))) (.AmbosLados (Utilities|Struct|BreakEstructuraObjeto _array_element_3)) (.x (.Distancia_Spawn (Utilities|Struct|BreakEstructuraObjeto _array_element_3))) (.y (.Distancia_Spawn (Utilities|Struct|BreakEstructuraObjeto _array_element_3))) (.Colores (Utilities|Struct|BreakEstructuraObjeto _array_element_3)) (.AplicarShader (Utilities|Struct|BreakEstructuraObjeto _array_element_3)))))))
    (:then_3
      ;[1 1 1] Casas Sub1 a Sub2 a Sub3
      (if (Variables|/Game/AuthenticationUI/OurGSGameMode.OurGSGameMode_C|GetSubnivel2Cargado _asour_gsgame_mode)
        (bind _aparicion__6 (CallFunction|ProbabilidadAparecimiento (Variables|/Game/AuthenticationUI/OurGSGameMode.OurGSGameMode_C|GetProbabilidadSubnivel2 _asour_gsgame_mode))) ; Reducir casas sub 2
        (if _aparicion__6
          (ControlCasas_Objetos()|GenerarCasas (.espaciousado (.OutItem (Utilities|Array|Random (Variables|/Game/AuthenticationUI/OurGSGameMode.OurGSGameMode_C|GetArregloEdificiosSub2 _asour_gsgame_mode)))) (.malla (.OutItem (Utilities|Array|Random (Variables|/Game/AuthenticationUI/OurGSGameMode.OurGSGameMode_C|GetArregloEdificiosSub2 _asour_gsgame_mode)))) (.colores (.OutItem (Utilities|Array|Random (Variables|/Game/AuthenticationUI/OurGSGameMode.OurGSGameMode_C|GetArregloEdificiosSub2 _asour_gsgame_mode)))) (.aplicarshader (.OutItem (Utilities|Array|Random (Variables|/Game/AuthenticationUI/OurGSGameMode.OurGSGameMode_C|GetArregloEdificiosSub2 _asour_gsgame_mode)))) :!label _label)
          (else
            (ControlCasas_Objetos()|GenerarCasas (.espaciousado (.OutItem (Utilities|Array|Random (Variables|/Game/AuthenticationUI/OurGSGameMode.OurGSGameMode_C|GetArregloEdificiosSub3 _asour_gsgame_mode)))) (.malla (.OutItem (Utilities|Array|Random (Variables|/Game/AuthenticationUI/OurGSGameMode.OurGSGameMode_C|GetArregloEdificiosSub3 _asour_gsgame_mode)))) (.colores (.OutItem (Utilities|Array|Random (Variables|/Game/AuthenticationUI/OurGSGameMode.OurGSGameMode_C|GetArregloEdificiosSub3 _asour_gsgame_mode)))) (.aplicarshader (.OutItem (Utilities|Array|Random (Variables|/Game/AuthenticationUI/OurGSGameMode.OurGSGameMode_C|GetArregloEdificiosSub3 _asour_gsgame_mode)))))))
        (else
          (bind _aparicion__7 (CallFunction|ProbabilidadAparecimiento (Variables|/Game/AuthenticationUI/OurGSGameMode.OurGSGameMode_C|GetProbabilidadSubnivel1 _asour_gsgame_mode)))
          (if _aparicion__7
            (ControlCasas_Objetos()|GenerarCasas "NewEnumerator4" (.malla (.OutItem (Utilities|Array|Random (Variables|/Game/AuthenticationUI/OurGSGameMode.OurGSGameMode_C|GetCasasSubnivel1_Strc _asour_gsgame_mode)))) (.colores (.OutItem (Utilities|Array|Random (Variables|/Game/AuthenticationUI/OurGSGameMode.OurGSGameMode_C|GetCasasSubnivel1_Strc _asour_gsgame_mode)))) (.aplicarshader (.OutItem (Utilities|Array|Random (Variables|/Game/AuthenticationUI/OurGSGameMode.OurGSGameMode_C|GetCasasSubnivel1_Strc _asour_gsgame_mode)))))
            (else
              (goto _label))))))))

(fn SpawnDecalsSubnivel
  (params (ArregloDecals :type Array%20of%20Estructura%20Decal%20Structures))
  (bind _outitem (Utilities|Array|Random ArregloDecals))
  (bind _guiacentro (Variables|Default|GetGuiaCentro))
  (bind _returnvalue (Math|Random|RandomFloatinRange (.x (.sizerange _outitem)) (.y (.sizerange _outitem))))
  (bind _returnvalue_2 (Transformation|GetWorldLocation _guiacentro))
  (for _index (range 0 (Math|Random|RandomIntegerinRange (.x (.numspawn _outitem)) (.y (.numspawn _outitem))))
    (bind _aparicion_ (CallFunction|ProbabilidadAparecimiento (.probabilidad _outitem)))
    (if _aparicion_
      (Rendering|Decal|SpawnDecalatLocation (.decalmaterial _outitem) (Math|Vector|MakeVector 1e+02 _returnvalue _returnvalue) (Math|Vector|MakeVector (+ (Math|Random|RandomFloatinRange -2.5e+02 2.5e+02) (.x _returnvalue_2)) (+ (.y _returnvalue_2) (Math|Random|RandomFloatinRange -2.5e+02 2.5e+02)) (.z _returnvalue_2)) (Math|Rotator|MakeRotator 0.0 -9e+01 (Math|Random|RandomFloatinRange 0.0 3.6e+02)) 0.0))))

(fn SpawnDecals
  (bind _asour_gsgame_mode (Utilities|Casting|CastToOurGSGameMode (Game|GetGameMode)))
  (if (Variables|/Game/AuthenticationUI/OurGSGameMode.OurGSGameMode_C|GetSubnivel2Cargado _asour_gsgame_mode)
    (bind _aparicion_ (CallFunction|ProbabilidadAparecimiento (Variables|/Game/AuthenticationUI/OurGSGameMode.OurGSGameMode_C|GetProbabilidadSubnivel2 _asour_gsgame_mode)))
    (if _aparicion_
      (CallFunction|SpawnDecalsSubnivel (Variables|/Game/AuthenticationUI/OurGSGameMode.OurGSGameMode_C|GetDecalsSubnivel2 _asour_gsgame_mode) :!label _label)
      (else
        (CallFunction|SpawnDecalsSubnivel (Variables|/Game/AuthenticationUI/OurGSGameMode.OurGSGameMode_C|GetDecalsSubnivel3 _asour_gsgame_mode))))
    (else
      (bind _aparicion__2 (CallFunction|ProbabilidadAparecimiento (Variables|/Game/AuthenticationUI/OurGSGameMode.OurGSGameMode_C|GetProbabilidadSubnivel1 _asour_gsgame_mode)))
      (if _aparicion__2
        (CallFunction|SpawnDecalsSubnivel (Variables|/Game/AuthenticationUI/OurGSGameMode.OurGSGameMode_C|GetDecalsSubnivel1 _asour_gsgame_mode))
        (else
          (goto _label))))))