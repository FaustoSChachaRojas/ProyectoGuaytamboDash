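; Plaza level piece for a runner game: a one-way lap circuit with chasers and a victory finale.
; Corner boxes play turn animations, move a blocking wall and toggle each other's overlaps; some activate the chasers.
; Box4 counts laps in InstanceHud, finally disabling input, destroying chasers, showing the winner widget, switching camera and starting delay-throttled random Niagara fireworks from Tick.
; A volume hides houses during overlap, restoring them on exit.
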(event OnComponentBeginOverlap(Box)
  (params (OverlappedComponent :type Primitive%20Component%20Object%20Reference) (OtherActor :type Actor%20Object%20Reference) (OtherComp :type Primitive%20Component%20Object%20Reference) (OtherBodyIndex :type Integer) (bFromSweep :type Boolean) (SweepResult :type Hit%20Result%20Structure%20%28by%20ref%29))
  (bind _asrun_character (Utilities|Casting|CastToRunCharacter OtherActor))
  (Default|AnimacionGiroDerecho _asrun_character)
  (Utilities|FlowControl|Delay 0.2)
  (Components|DestroyComponent (Variables|Default|GetBox)))

(event OnComponentBeginOverlap(Box1)
  (params (OverlappedComponent :type Primitive%20Component%20Object%20Reference) (OtherActor :type Actor%20Object%20Reference) (OtherComp :type Primitive%20Component%20Object%20Reference) (OtherBodyIndex :type Integer) (bFromSweep :type Boolean) (SweepResult :type Hit%20Result%20Structure%20%28by%20ref%29))
  (bind _asrun_character (Utilities|Casting|CastToRunCharacter OtherActor))
  (Default|AnimacionGiroIzquierdo _asrun_character)
  (Utilities|FlowControl|Delay 0.2)
  (CallFunction|ControlUnaDireccion (Variables|Default|GetBox1) (Variables|Default|GetBox4))
  (Utilities|FlowControl|Delay 1.0)
  (Variables|/Game/Mannequin/Character/Mesh/Toro/Toro_BP2.Toro_BP2_C|SetPersiguir (Variables|Default|GetPerseguir) true)
  (bind _asinstance_hud (Utilities|Casting|CastToInstanceHud (Game|GetGameInstance)))
  (Variables|/Game/Runner_Files/UI/RaymiÑam/InstanceHud.InstanceHud_C|SetMostrarLaps _asinstance_hud true))

(event OnComponentBeginOverlap(Box2)
  (params (OverlappedComponent :type Primitive%20Component%20Object%20Reference) (OtherActor :type Actor%20Object%20Reference) (OtherComp :type Primitive%20Component%20Object%20Reference) (OtherBodyIndex :type Integer) (bFromSweep :type Boolean) (SweepResult :type Hit%20Result%20Structure%20%28by%20ref%29))
  (bind _asrun_character (Utilities|Casting|CastToRunCharacter OtherActor))
  (Default|AnimacionGiroIzquierdo _asrun_character)
  (Utilities|FlowControl|Delay 0.2)
  (CallFunction|ControlUnaDireccion (Variables|Default|GetBox2) (Variables|Default|GetBox1)))

(event OnComponentBeginOverlap(Box3)
  (params (OverlappedComponent :type Primitive%20Component%20Object%20Reference) (OtherActor :type Actor%20Object%20Reference) (OtherComp :type Primitive%20Component%20Object%20Reference) (OtherBodyIndex :type Integer) (bFromSweep :type Boolean) (SweepResult :type Hit%20Result%20Structure%20%28by%20ref%29))
  (bind _asrun_character (Utilities|Casting|CastToRunCharacter OtherActor))
  (Variables|/Game/Mannequin/Character/Mesh/Toro/Toro_BP2.Toro_BP2_C|SetPersiguir (Variables|Default|GetPerseguir2) true)
  (Default|AnimacionGiroIzquierdo _asrun_character)
  (Utilities|FlowControl|Delay 0.2)
  (CallFunction|ControlUnaDireccion (Variables|Default|GetBox3) (Variables|Default|GetBox2)))

(event OnComponentBeginOverlap(Box4)
  (params (OverlappedComponent :type Primitive%20Component%20Object%20Reference) (OtherActor :type Actor%20Object%20Reference) (OtherComp :type Primitive%20Component%20Object%20Reference) (OtherBodyIndex :type Integer) (bFromSweep :type Boolean) (SweepResult :type Hit%20Result%20Structure%20%28by%20ref%29))
  (bind _perseguir2 (Variables|Default|GetPerseguir2))
  (bind _perseguir (Variables|Default|GetPerseguir))
  (bind _asrun_character (Utilities|Casting|CastToRunCharacter OtherActor))
  (Default|AnimacionGiroIzquierdo _asrun_character)
  (Utilities|FlowControl|Delay 0.2)
  (CallFunction|ControlUnaDireccion (Variables|Default|GetBox4) (Variables|Default|GetBox3))
  (bind _asinstance_hud (Utilities|Casting|CastToInstanceHud (Game|GetGameInstance)))
  (if (== (Variables|/Game/Runner_Files/UI/RaymiÑam/InstanceHud.InstanceHud_C|GetNumeroLaps _asinstance_hud) 3)
    (Variables|Default|SetActivarFuegos true)
    (Input|DisableInput (Game|GetPlayerCharacter 0) (Game|GetPlayerController 0))
    (Utilities|FlowControl|Sequence
      (:then_0
        (Variables|/Game/Mannequin/Character/Mesh/Toro/Toro_BP2.Toro_BP2_C|SetPersiguir _perseguir false)
        (Actor|DestroyActor _perseguir)
        (bind _returnvalue (UserInterface|CreateWidget "/Game/Runner_Files/UI/RaymiÑam/Winner/Winner_BP.Winner_BP_C"))
        (Utilities|FlowControl|Delay 0.4)
        (UserInterface|Viewport|AddtoViewport _returnvalue 0)
        (bind _asrun_character_2 (Utilities|Casting|CastToRunCharacter (Game|Player|GetPlayerPawn 0)))
        (Variables|/Game/RunnerPersonBP/Blueprints/RunCharacter.RunCharacter_C|SetBlend%20Time _asrun_character_2 1.0)
        (Variables|/Game/RunnerPersonBP/Blueprints/RunCharacter.RunCharacter_C|SetCurrentCamera _asrun_character_2 3)
        (Default|SwitchCamera _asrun_character_2)
        (Variables|/Script/Engine.CharacterMovementComponent|SetMaxWalkSpeed (Variables|/Script/Engine.Character|GetCharacterMovement _asrun_character_2) 7e+01)
        (bind _asinstance_hud_2 (Utilities|Casting|CastToInstanceHud (Game|GetGameInstance)))
        (Variables|/Game/Runner_Files/UI/RaymiÑam/InstanceHud.InstanceHud_C|SetMostrarLaps _asinstance_hud_2 false)
        (Variables|/Game/Runner_Files/UI/RaymiÑam/InstanceHud.InstanceHud_C|SetNumeroLaps _asinstance_hud_2 4))
      (:then_1
        (Variables|/Game/Mannequin/Character/Mesh/Toro/Toro_BP2.Toro_BP2_C|SetPersiguir _perseguir2 false)
        (Actor|DestroyActor _perseguir2)))
    (else
      (bind _output_get (Variables|/Game/Runner_Files/UI/RaymiÑam/InstanceHud.InstanceHud_C|SetNumeroLaps _asinstance_hud (+ (Variables|/Game/Runner_Files/UI/RaymiÑam/InstanceHud.InstanceHud_C|GetNumeroLaps _asinstance_hud) 1)))
      (Development|PrintString (Utilities|String|Append "Vuelta No: " (Utilities|String|ToString(Integer) _output_get)) true true "(R=1.000000,G=0.000000,B=0.029223,A=1.000000)" 2e+01))))

(event OnComponentBeginOverlap(ShowHideHousesVolume)
  (params (OverlappedComponent :type Primitive%20Component%20Object%20Reference) (OtherActor :type Actor%20Object%20Reference) (OtherComp :type Primitive%20Component%20Object%20Reference) (OtherBodyIndex :type Integer) (bFromSweep :type Boolean) (SweepResult :type Hit%20Result%20Structure%20%28by%20ref%29))
  ;[0 0 0] Encender y apagar casas
  (Rendering|SetVisibility (Variables|Default|GetCasa_n3_08_Child2) false false))

(event OnComponentEndOverlap(ShowHideHousesVolume)
  (params (OverlappedComponent :type Primitive%20Component%20Object%20Reference) (OtherActor :type Actor%20Object%20Reference) (OtherComp :type Primitive%20Component%20Object%20Reference) (OtherBodyIndex :type Integer))
  ;[0 0 0] Encender y apagar casas
  (Rendering|SetVisibility (Variables|Default|GetCasa_n3_08_Child2) true false)
  (Components|DestroyComponent (Variables|Default|GetShowHideHousesVolume)))

(event EventBeginPlay)

(event Collision|EventActorBeginOverlap
  (params (OtherActor :type Actor%20Object%20Reference)))

(event EventTick
  (params (DeltaSeconds :type Float%20%28single-precision%29))
  (if (Variables|Default|GetActivarFuegos)
    (Utilities|FlowControl|Delay 1.0)
    (CallFunction|FuegosArtificiales)))

(fn ConstructionScript)

(fn ControlUnaDireccion
  (params (BoxCollisionActual :type Box%20Component%20Object%20Reference) (BoxCollisionPrevio :type Box%20Component%20Object%20Reference))
  (Transformation|SetWorldTransform (Variables|Default|Getmuro) (Transformation|GetWorldTransform BoxCollisionActual) false false)
  (Variables|/Script/Engine.PrimitiveComponent|SetbGenerateOverlapEvents BoxCollisionActual false)
  (Variables|/Script/Engine.PrimitiveComponent|SetbGenerateOverlapEvents BoxCollisionPrevio true))

(fn FuegosArtificiales
  (Utilities|FlowControl|Sequence
    (:then_0
      (bind _returnvalue (Niagara|SpawnSystematLocation "/Game/Runner_Files/VFX_F/Fireworks/FArtificialEmitter_System.FArtificialEmitter_System" (Math|Vector|MakeVector (Math|Random|RandomFloatinRange 5e+03 1.5e+04) (Math|Random|RandomFloatinRange -1e+04 5e+03) -5e+03)))
      (Niagara|SetNiagaraVariable(LinearColor) _returnvalue "Color" (Utilities|Struct|MakeLinearColor (Math|Random|RandomFloatinRange -2e+01 2e+01) (Math|Random|RandomFloatinRange -2e+01 2e+01) (Math|Random|RandomFloatinRange -2e+01 1.0) 1.0)))
    (:then_1
      (bind _returnvalue_2 (Niagara|SpawnSystematLocation "/Game/Runner_Files/VFX_F/Fireworks/FArtificialEmitter_System.FArtificialEmitter_System" (Math|Vector|MakeVector (Math|Random|RandomFloatinRange 1e+04 1.5e+04) (Math|Random|RandomFloatinRange -7.5e+03 7.5e+03) -2e+03) "0.000000,1.000000,1.000000"))
      (Niagara|SetNiagaraVariable(LinearColor) _returnvalue_2 "Color" (Utilities|Struct|MakeLinearColor (Math|Random|RandomFloatinRange -2e+01 2e+01) (Math|Random|RandomFloatinRange -2e+01 2e+01) (Math|Random|RandomFloatinRange -2e+01 1.0) 1.0)))
    (:then_2
      (bind _returnvalue_3 (Niagara|SpawnSystematLocation "/Game/Runner_Files/VFX_F/Fireworks/FArtificialEmitter_System.FArtificialEmitter_System" (Math|Vector|MakeVector (Math|Random|RandomFloatinRange 1e+04 1.5e+04) (Math|Random|RandomFloatinRange -5e+03 1e+04) -2e+03)))
      (Niagara|SetNiagaraVariable(LinearColor) _returnvalue_3 "Color" (Utilities|Struct|MakeLinearColor (Math|Random|RandomFloatinRange -2e+01 2e+01) (Math|Random|RandomFloatinRange -2e+01 2e+01) (Math|Random|RandomFloatinRange -2e+01 1.0) 1.0)))))