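; Fruit pickup in the Semillas (seeds) set of the runner, with a mesh picked randomly on construction.
; With the magnet active, entering BigSphere pulls it toward the player and collects it after a delay; touching it collects directly.
; Collection adds game-mode coins, calls PasoNivel on multiples of the active sublevel's divisor, destroys it and updates InstanceHud.
; Direct touch also pauses for a one-time SemillaHud popup.
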(event OnComponentBeginOverlap(BigSphere)
  (params (OverlappedComponent :type Primitive%20Component%20Object%20Reference) (OtherActor :type Actor%20Object%20Reference) (OtherComp :type Primitive%20Component%20Object%20Reference) (OtherBodyIndex :type Integer) (bFromSweep :type Boolean) (SweepResult :type Hit%20Result%20Structure%20%28by%20ref%29))
  (bind _asrun_character (Utilities|Casting|CastToRunCharacter OtherActor))
  (if (Variables|/Game/RunnerPersonBP/Blueprints/RunCharacter.RunCharacter_C|GetMagnetActive _asrun_character)
    (Utilities|FlowControl|Sequence
      (:then_0
        (Timeline|Timeline_0 Play
          (:Update
            (Transformation|SetWorldLocation (Variables|Default|GetCoin) (Math|Interpolation|VInterpTo (Transformation|GetWorldLocation (Variables|Default|GetCoin)) (Transformation|GetActorLocation (Game|GetPlayerCharacter 0)) (Utilities|Time|GetWorldDeltaSeconds) 5.0) false false))))
      (:then_1
        (Utilities|FlowControl|Delay 0.8)
        (bind _asour_gsgame_mode (Utilities|Casting|CastToOurGSGameMode (Game|GetGameMode)))
        (bind _output_get (Variables|/Game/AuthenticationUI/OurGSGameMode.OurGSGameMode_C|SetCoins _asour_gsgame_mode (+ (Variables|/Game/AuthenticationUI/OurGSGameMode.OurGSGameMode_C|GetCoins _asour_gsgame_mode) 15)))
        (if (Variables|/Game/AuthenticationUI/OurGSGameMode.OurGSGameMode_C|GetSubnivel1Activo _asour_gsgame_mode)
          (Variables|Default|SetRestoDivision 10)
          (if (== (Math|Integer|%(Integer) _output_get (Variables|Default|GetRestoDivision)) 0) :!label _label
            (Default|PasoNivel _asour_gsgame_mode))
          (Actor|DestroyActor)
          (bind _asinstance_hud (Utilities|Casting|CastToInstanceHud (Game|GetGameInstance)))
          (Variables|/Game/Runner_Files/UI/RaymiÑam/InstanceHud.InstanceHud_C|SetSemillas _asinstance_hud (Variables|/Game/AuthenticationUI/OurGSGameMode.OurGSGameMode_C|GetCoins _asour_gsgame_mode))
          (elif (Variables|/Game/AuthenticationUI/OurGSGameMode.OurGSGameMode_C|GetSubnivel2Activo _asour_gsgame_mode)
            (Variables|Default|SetRestoDivision 20)
            (goto _label)
            (elif (Variables|/Game/AuthenticationUI/OurGSGameMode.OurGSGameMode_C|GetSubnivel3Activo _asour_gsgame_mode)
              (Variables|Default|SetRestoDivision 30)
              (goto _label))))))))

(event OnComponentBeginOverlap(Coin)
  (params (OverlappedComponent :type Primitive%20Component%20Object%20Reference) (OtherActor :type Actor%20Object%20Reference) (OtherComp :type Primitive%20Component%20Object%20Reference) (OtherBodyIndex :type Integer) (bFromSweep :type Boolean) (SweepResult :type Hit%20Result%20Structure%20%28by%20ref%29))
  (Utilities|Casting|CastToRunCharacter OtherActor)
  (Utilities|FlowControl|Sequence
    (:then_0
      (bind _asour_gsgame_mode (Utilities|Casting|CastToOurGSGameMode (Game|GetGameMode)))
      (bind _output_get (Variables|/Game/AuthenticationUI/OurGSGameMode.OurGSGameMode_C|SetCoins _asour_gsgame_mode (+ (Variables|/Game/AuthenticationUI/OurGSGameMode.OurGSGameMode_C|GetCoins _asour_gsgame_mode) 15)))
      (if (Variables|/Game/AuthenticationUI/OurGSGameMode.OurGSGameMode_C|GetSubnivel1Activo _asour_gsgame_mode)
        (Variables|Default|SetRestoDivision 10)
        (if (== (Math|Integer|%(Integer) _output_get (Variables|Default|GetRestoDivision)) 0) :!label _label
          (Default|PasoNivel _asour_gsgame_mode))
        (Actor|DestroyActor)
        (bind _asinstance_hud (Utilities|Casting|CastToInstanceHud (Game|GetGameInstance)))
        (Variables|/Game/Runner_Files/UI/RaymiÑam/InstanceHud.InstanceHud_C|SetSemillas _asinstance_hud (Variables|/Game/AuthenticationUI/OurGSGameMode.OurGSGameMode_C|GetCoins _asour_gsgame_mode))
        (elif (Variables|/Game/AuthenticationUI/OurGSGameMode.OurGSGameMode_C|GetSubnivel2Activo _asour_gsgame_mode)
          (Variables|Default|SetRestoDivision 20)
          (goto _label)
          (elif (Variables|/Game/AuthenticationUI/OurGSGameMode.OurGSGameMode_C|GetSubnivel3Activo _asour_gsgame_mode)
            (Variables|Default|SetRestoDivision 30)
            (goto _label)))))
    (:then_1
      (bind _asinstance_hud_2 (Utilities|Casting|CastToInstanceHud (Game|GetGameInstance)))
      (if (Math|Boolean|Equal(Boolean) (Variables|/Game/Runner_Files/UI/RaymiÑam/InstanceHud.InstanceHud_C|GetDesactiveHudsSemilla _asinstance_hud_2) false)
        (Game|SetGamePaused true)
        (bind _returnvalue (UserInterface|CreateWidget "/Game/Runner_Files/UI/RaymiÑam/HUD-TUTO/SemillaHud.SemillaHud_C"))
        (UserInterface|Viewport|AddtoViewport _returnvalue 0)
        (Variables|/Game/Runner_Files/UI/RaymiÑam/InstanceHud.InstanceHud_C|SetDesactiveHudsSemilla _asinstance_hud_2 true)))))

(fn ConstructionScript
  (Components|StaticMesh|SetStaticMesh (Variables|Default|GetCoin) (.OutItem (Utilities|Array|Random (Variables|Default|GetMallas)))))