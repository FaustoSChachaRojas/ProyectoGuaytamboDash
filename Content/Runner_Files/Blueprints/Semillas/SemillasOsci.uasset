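; SemillasOsci is a runner-game spawner actor that lays out a row of semilla (seed) pickups or objects in an oscillating pattern.
; On BeginPlay it spawns a fixed series of semilla actors at even steps along world X from its Arrow component.
; A sine of the loop index offsets each one in Y, forming a static wave at constant height.
; Each spawned actor attaches to the spawner, keeping its world location.
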(event EventBeginPlay
  (CallFunction|SpawnSemillasOsci))

(event Collision|EventActorBeginOverlap
  (params (OtherActor :type Actor%20Object%20Reference)))

(event EventTick
  (params (DeltaSeconds :type Float%20%28single-precision%29)))

(fn ConstructionScript)

(fn SpawnSemillasOsci
  (bind _arrow (Variables|Default|GetArrow))
  (bind _returnvalue (Transformation|GetWorldLocation _arrow))
  (LocalVariables|SettempX (.x _returnvalue))
  (for _index (range 0 14)
    (bind _output_get (LocalVariables|SettempX (+ (LocalVariables|GettempX) 125.0)))
    (bind _returnvalue_2 (Game|SpawnActorfromClass "/Game/Runner_Files/Blueprints/Semillas/Semilla_BP.Semilla_BP_C" (Math|Transform|MakeTransform (Math|Vector|MakeVector _output_get (+ (* (Math|Trig|Sin(Radians) (/ (Math|Conversions|ToFloat(Integer) _index) 3.0)) -2.5e+02) (.y _returnvalue)) (.z _returnvalue)) "0, 0, 0" "1,1,1") "Undefined" 0 0))
    (Transformation|AttachActorToActor _returnvalue_2 self "None" "KeepWorld" "KeepRelative" "KeepRelative" true)))